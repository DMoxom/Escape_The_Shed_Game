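; BP_NewInteractButton is a button that responds to interact input while PlayerNear is set by its ActivationTrigger overlap.
; Interacting calls Pressed whether or not Toggle is set.
; Without Toggle, it acts as a hold button, calling Released when the interaction ends nearby or an overlap with the trigger ends.
; The overlap events set PlayerNear without checking which actor overlaps.
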(event OnComponentBeginOverlap(ActivationTrigger)
  (params (OverlappedComponent :type Primitive%20Component%20Object%20Reference) (OtherActor :type Actor%20Object%20Reference) (OtherComp :type Primitive%20Component%20Object%20Reference) (OtherBodyIndex :type Integer) (bFromSweep :type Boolean) (SweepResult :type Hit%20Result%20Structure%20%28by%20ref%29))
  (Variables|Default|SetPlayerNear true))

(event OnComponentEndOverlap(ActivationTrigger)
  (params (OverlappedComponent :type Primitive%20Component%20Object%20Reference) (OtherActor :type Actor%20Object%20Reference) (OtherComp :type Primitive%20Component%20Object%20Reference) (OtherBodyIndex :type Integer))
  (Variables|Default|SetPlayerNear false)
  (if (not (Variables|Default|GetToggle?))
    (CallFunction|Released)))

(event Custom|Interacted
  (if (Variables|Default|GetPlayerNear)
    (if (Variables|Default|GetToggle?)
      (CallFunction|Pressed)
      (else
        (CallFunction|Pressed)))))

(event Custom|Interact%20End
  (if (Variables|Default|GetPlayerNear)
    (if (not (Variables|Default|GetToggle?))
      (CallFunction|Released))))

(fn ConstructionScript
  (|CallParentFunction))