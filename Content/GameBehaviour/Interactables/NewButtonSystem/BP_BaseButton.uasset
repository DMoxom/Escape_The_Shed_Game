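; BP_BaseButton is a base interactable button that supports toggle or hold behavior, gated by a Prerequisite flag.
; Pressed flips or sets IsPressed, and Released clears it for non-toggle buttons only.
; An optional use count decrements per press, prints for debugging and blocks the press notification once exhausted, though IsPressed still changes.
; State changes are forwarded by setting itself as the Activator's TargetButton and calling ButtonState.
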(event Custom|Pressed
  (bind _activator (Variables|Default|GetActivator))
  (if (Variables|Default|GetPrerequisite)
    (if (Variables|Default|GetToggle?)
      (Variables|Default|SetIsPressed? (not (Variables|Default|GetIsPressed?)))
      (else
        (Variables|Default|SetIsPressed? true)))
    (if (Variables|Default|GetHasCount?)
      (if (> (Variables|Default|GetUseCount) 0)
        (bind _result (Math|Integer|DecrementInt (Variables|Default|GetUseCount))
          (:%20%20
            (Variables|Default|SetUseCount _result)
            (Development|PrintString (Utilities|String|ToString(Integer) (Variables|Default|GetUseCount)))
            (Variables|/Game/GameBehaviour/Interactables/NewButtonSystem/BP_ActivatorBase.BP_ActivatorBase_C|SetTargetButton _activator self :!label _label)
            (Default|ButtonState _activator))))
      (else
        (goto _label)))))

(event Custom|Released
  (bind _activator (Variables|Default|GetActivator))
  (if (not (Variables|Default|GetToggle?))
    (Variables|Default|SetIsPressed? false)
    (Variables|/Game/GameBehaviour/Interactables/NewButtonSystem/BP_ActivatorBase.BP_ActivatorBase_C|SetTargetButton _activator self)
    (Default|ButtonState _activator)))

(fn ConstructionScript)