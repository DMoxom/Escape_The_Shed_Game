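; BP_BaseTargetedLaunch is a bounce pad that launches a BP_BasePlayer overlapping its Trigger, based on a TargetLocation actor.
; CalculateSpeed derives speed from the height difference to the target, using a projectile formula with a fixed angle and hardcoded 9.8 gravity.
; CalculateLaunch scales the normalized player-minus-target vector, which points away from the target, by that speed.
; LaunchCharacter applies the result, overriding existing velocity; debug prints show both values.
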(event OnComponentBeginOverlap(Trigger)
  (params (OverlappedComponent :type Primitive%20Component%20Object%20Reference) (OtherActor :type Actor%20Object%20Reference) (OtherComp :type Primitive%20Component%20Object%20Reference) (OtherBodyIndex :type Integer) (bFromSweep :type Boolean) (SweepResult :type Hit%20Result%20Structure%20%28by%20ref%29))
  (bind _target_location (Variables|Default|GetTarget%20Location))
  (bind _asbp_base_player (Utilities|Casting|CastToBP_BasePlayer OtherActor))
  (bind _speed (CallFunction|CalculateSpeed (- (.z (Transformation|GetActorLocation _target_location)) (.z (Transformation|GetActorLocation _asbp_base_player))) 45.0))
  (Development|PrintString (Utilities|String|ToString(Float) _speed))
  (bind _launchvelocity (CallFunction|CalculateLaunch (Transformation|GetActorLocation _target_location) _speed _asbp_base_player))
  (Development|PrintString (Utilities|String|ToString(Vector) _launchvelocity))
  (Character|LaunchCharacter _asbp_base_player _launchvelocity true true))

(fn ConstructionScript)

(fn CalculateLaunch
  (params (TargetLocation :type Vector) (LaunchSpeed :type Float%20%28double-precision%29) (Launchee :type Actor%20Object%20Reference))
  (return (* (Math|Vector|Normalize (- (Transformation|GetActorLocation Launchee) TargetLocation)) LaunchSpeed)))

(fn CalculateSpeed
  (params (H :type Float%20%28double-precision%29) (Theta%28Degrees%29 :type Float%20%28double-precision%29))
  (return (Math|Float|Sqrt (/ (* H 9.8) (Math|Trig|Sin(Radians) (* 2.0 (* Theta%28Degrees%29 (/ 3.14159 1.8e+02))))))))