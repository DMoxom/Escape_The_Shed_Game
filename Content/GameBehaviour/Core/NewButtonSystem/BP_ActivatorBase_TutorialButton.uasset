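; Tutorial activator in the button system that relocates both players based on the state of a target button.
; Its ButtonState event passes TargetButton to ButtonStateChange and acts only when that returns true.
; It then teleports player characters 0 and 1 to the Player1Location and Player2Location transforms, without sweeping.
; The construction script only calls the parent's.
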(event EventButtonState
  (bind _buttonstate (CallFunction|ButtonStateChange (Variables|Default|GetTargetButton)))
  (if _buttonstate
    (Transformation|SetActorTransform (Game|GetPlayerCharacter 0) (Variables|Default|GetPlayer1Location) false true)
    (Transformation|SetActorTransform (Game|GetPlayerCharacter 1) (Variables|Default|GetPlayer2Location) false true)))

(fn ConstructionScript
  (|CallParentFunction))