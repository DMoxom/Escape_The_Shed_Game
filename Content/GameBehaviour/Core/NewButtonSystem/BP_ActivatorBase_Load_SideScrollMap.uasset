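; Level-exit activator button that loads the side-scroll map once the players have all keys.
; On BeginPlay it caches the OptionsGameInstance and creates a loading-screen widget.
; When the button state fires it sets level progress to 2 and swaps in level 2 collectibles on the game instance.
; If keys are held, it shows the loading screen, removes both local players and their pawns, then opens SideScrollTestMap after a short delay.
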(event EventCanUseButton
  (params (haveKeys :type Boolean))
  (Variables|Default|SethaveAllKeys haveKeys))

(event EventButtonState
  (bind _optionsgameinstance (Variables|Default|GetOptionsGameInstance))
  (bind _optionsgameinstance_2 (Variables|Default|GetOptionsGameInstance))
  (Variables|/Game/GameBehaviour/Core/GameInstance/OptionsGameInstance.OptionsGameInstance_C|SetMaxLevelReached _optionsgameinstance_2 2)
  (Variables|/Game/GameBehaviour/Core/GameInstance/OptionsGameInstance.OptionsGameInstance_C|SetCurrentLevel _optionsgameinstance_2 2)
  (Variables|/Game/GameBehaviour/Core/GameInstance/OptionsGameInstance.OptionsGameInstance_C|SetCollectibles _optionsgameinstance (Variables|/Game/GameBehaviour/Core/GameInstance/OptionsGameInstance.OptionsGameInstance_C|GetCollectiblesLevel2 _optionsgameinstance))
  (if (Variables|Default|GethaveAllKeys)
    (CallFunction|LoadingScreen (Variables|Default|GetLoadingScreenBP))
    (Class|GameplayStatics|RemovePlayer (Game|GetPlayerController 0) true)
    (Class|GameplayStatics|RemovePlayer (Game|GetPlayerController 1) true)
    (Utilities|FlowControl|Delay 3.0)
    (Game|OpenLevel(byObjectReference) "/Game/GameBehaviour/Maps/Testing/SideScrollTestMap.SideScrollTestMap")))

(event EventBeginPlay
  (bind _asoptions_game_instance (Utilities|Casting|CastToOptionsGameInstance (Game|GetGameInstance)))
  (Variables|Default|SetOptionsGameInstance _asoptions_game_instance)
  (bind _returnvalue (UserInterface|CreateWidget "/Game/GameBehaviour/UI/LoadingScreen/BP_LoadingScreen.BP_LoadingScreen_C" (Game|GetPlayerController 0)))
  (Variables|Default|SetLoadingScreenBP _returnvalue))

(fn ConstructionScript
  (|CallParentFunction))