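; BP_PressureButton is a pressure-triggered button that activates when enough players stand inside its PresureTrigger component.
; Overlap begin and end events raise or lower PlayerCount for actors tagged "Player" and print the count.
; It calls Pressed when the count equals MinPlayers and Released on any end overlap that leaves it below that threshold.
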(event OnComponentBeginOverlap(Presuretrigger)
  (params (OverlappedComponent :type Primitive%20Component%20Object%20Reference) (OtherActor :type Actor%20Object%20Reference) (OtherComp :type Primitive%20Component%20Object%20Reference) (OtherBodyIndex :type Integer) (bFromSweep :type Boolean) (SweepResult :type Hit%20Result%20Structure%20%28by%20ref%29))
  (for _array_element (Utilities|Array|MakeArray OtherActor)
    (if (Actor|ActorHasTag _array_element "Player")
      (bind _result (Math|Integer|IncrementInt (Variables|Default|GetPlayer%20Count))
        (:%20%20
          (Variables|Default|SetPlayer%20Count _result)))))
  (Development|PrintString (Utilities|String|ToString(Integer) (Variables|Default|GetPlayer%20Count)))
  (if (== (Variables|Default|GetPlayer%20Count) (Variables|Default|GetMinPlayers))
    (CallFunction|Pressed)))

(event OnComponentEndOverlap(Presuretrigger)
  (params (OverlappedComponent :type Primitive%20Component%20Object%20Reference) (OtherActor :type Actor%20Object%20Reference) (OtherComp :type Primitive%20Component%20Object%20Reference) (OtherBodyIndex :type Integer))
  (for _array_element (Utilities|Array|MakeArray OtherActor)
    (if (Actor|ActorHasTag _array_element "Player")
      (bind _result (Math|Integer|DecrementInt (Variables|Default|GetPlayer%20Count))
        (:%20%20
          (Variables|Default|SetPlayer%20Count _result)))))
  (Development|PrintString (Utilities|String|ToString(Integer) (Variables|Default|GetPlayer%20Count)))
  (if (< (Variables|Default|GetPlayer%20Count) (Variables|Default|GetMinPlayers))
    (CallFunction|Released)))

(fn ConstructionScript
  (|CallParentFunction))