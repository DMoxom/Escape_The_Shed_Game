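; BP_StandButton is a floor-style button that sets IsOn when a BP_BasePlayer overlaps its PlayerTrigger, gated by PrerequisiteMet and an optional use limit.
; In toggle mode each entry flips IsOn and decrements any positive ReaminingUses, even when HasUseLimit is off.
; Otherwise IsOn holds true until the player leaves, and a limited use is spent on release.
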(event OnComponentBeginOverlap(PlayerTrigger)
  (params (OverlappedComponent :type Primitive%20Component%20Object%20Reference) (OtherActor :type Actor%20Object%20Reference) (OtherComp :type Primitive%20Component%20Object%20Reference) (OtherBodyIndex :type Integer) (bFromSweep :type Boolean) (SweepResult :type Hit%20Result%20Structure%20%28by%20ref%29))
  ;[1 1 1] When Button is pressed
  (Utilities|Casting|CastToBP_BasePlayer OtherActor)
  (if (Variables|Default|GetPrerequisite%20met?)
    (if (Variables|Default|GetHasUseLimit?)
      (if (> (Variables|Default|GetReaminingUses) 0)
        (if (Variables|Default|GetTogglable?) :!label _label
          (Variables|Default|SetIsOn? (not (Variables|Default|GetIsOn?)))
          (if (> (Variables|Default|GetReaminingUses) 0)
            (bind _result (Math|Integer|DecrementInt (Variables|Default|GetReaminingUses))
              (:%20%20
                (Variables|Default|SetReaminingUses _result))))
          (else
            (Variables|Default|SetIsOn? true))))
      (else
        (goto _label)))))

(event OnComponentEndOverlap(PlayerTrigger)
  (params (OverlappedComponent :type Primitive%20Component%20Object%20Reference) (OtherActor :type Actor%20Object%20Reference) (OtherComp :type Primitive%20Component%20Object%20Reference) (OtherBodyIndex :type Integer))
  ;[1 1 1] When Button is unpressed
  (Utilities|Casting|CastToBP_BasePlayer OtherActor)
  (if (not (Variables|Default|GetTogglable?))
    (if (Variables|Default|GetPrerequisite%20met?)
      (if (Variables|Default|GetHasUseLimit?)
        (if (> (Variables|Default|GetReaminingUses) 0)
          (bind _result (Math|Integer|DecrementInt (Variables|Default|GetReaminingUses))
            (:%20%20
              (Variables|Default|SetReaminingUses _result)
              (Variables|Default|SetIsOn? false :!label _label))))
        (else
          (goto _label))))))

(event EventBeginPlay
  (Variables|Default|SetIsOn? false))

(fn ConstructionScript)