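; Bounce pad that fakes a launch by carrying an overlapping Player 1 or Player 2 along a spline.
; The box overlap stores the player, plays the pump press animation and runs a timeline scaled to LaunchTime.
; Each update sets the player's location by spline distance, without sweep or physics impulse.
; On finish, the timeline rewinds, the player's end position is reapplied, and box collision is briefly disabled.
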(event OnComponentBeginOverlap(Box)
  (params (OverlappedComponent :type Primitive%20Component%20Object%20Reference) (OtherActor :type Actor%20Object%20Reference) (OtherComp :type Primitive%20Component%20Object%20Reference) (OtherBodyIndex :type Integer) (bFromSweep :type Boolean) (SweepResult :type Hit%20Result%20Structure%20%28by%20ref%29))
  ;[1 1 1] Identifies player to launch
  (bind _asbp_player_1 (Utilities|Casting|CastToBP_Player1 OtherActor)
    (:then
      (Variables|Default|SetAs%20BP%20Base%20Player _asbp_player_1))
    (:CastFailed
      (bind _asbp_player_2 (Utilities|Casting|CastToBP_Player2 OtherActor))
      (Variables|Default|SetAs%20BP%20Base%20Player _asbp_player_2)))
  (CallFunction|Launch))

(event Custom|Launch
  (bind _box (Variables|Default|GetBox))
  (bind _as_bp_base_player (Variables|Default|GetAs%20BP%20Base%20Player))
  (bind _spline (Variables|Default|GetSpline))
  (Components|Animation|PlayAnimation (Variables|Default|GetSkeletalMesh) "/Game/GameBehaviour/Art/Anims/Pump_press_anim_Anim_Montage.Pump_press_anim_Anim_Montage" false)
  (bind _move_track (Timeline|PlayerLaunch Play)
    (:Update
      (Transformation|SetActorLocation _as_bp_base_player (Spline|GetLocationatDistanceAlongSpline (Variables|Default|GetSpline) (Math|Float|Lerp 0.0 (Spline|GetDistanceAlongSplineatSplinePoint _spline (- (Spline|GetNumberOfSplinePoints _spline) 1)) _move_track) "World") false false))
    (:Finished
      (bind _output_get (Variables|Default|SetPostionBuffer (Transformation|GetActorLocation (Variables|Default|GetAs%20BP%20Base%20Player))))
      (Collision|SetCollisionEnabled _box "NoCollision")
      (Components|Timeline|SetNewTime (Variables|Default|GetPlayerLaunch) 0.0)
      (Transformation|SetActorLocation _as_bp_base_player _output_get false false)
      (Utilities|FlowControl|Delay 0.2)
      (Collision|SetCollisionEnabled _box "QueryOnly"))))

(event EventBeginPlay
  (Components|Timeline|SetPlayRate (Variables|Default|GetPlayerLaunch) (/ 1.0 (Variables|Default|GetLaunchTime))))

(fn ConstructionScript)