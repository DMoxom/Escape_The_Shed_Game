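; Base launch volume, or bounce pad, that flings the player in a set direction on entering its trigger.
; On overlap, a BP_BasePlayer is launched along the Arrow's forward vector scaled by LaunchForce, replacing its existing velocity on all axes.
; When OverideTrajectory is set, BeginPlay applies only the rotation of ArrowTransform to the Arrow, allowing per-instance launch directions.
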(event OnComponentBeginOverlap(Trigger)
  (params (OverlappedComponent :type Primitive%20Component%20Object%20Reference) (OtherActor :type Actor%20Object%20Reference) (OtherComp :type Primitive%20Component%20Object%20Reference) (OtherBodyIndex :type Integer) (bFromSweep :type Boolean) (SweepResult :type Hit%20Result%20Structure%20%28by%20ref%29))
  (bind _asbp_base_player (Utilities|Casting|CastToBP_BasePlayer OtherActor))
  (Character|LaunchCharacter _asbp_base_player (* (Math|Vector|GetForwardVector (Variables|Default|GetArrow)) (Variables|Default|GetLaunch%20Force)) true true))

(event EventBeginPlay
  (bind _arrow (Variables|Default|GetArrow))
  (bind _returnvalue (Transformation|GetWorldTransform _arrow))
  ;[1 1 1] Arrow Orientation Setup
  (if (Variables|Default|GetOveride%20Trajectory)
    (Transformation|SetWorldTransform _arrow (Math|Transform|MakeTransform (.location _returnvalue) (.rotation (Variables|Default|GetArrowTransform)) (.scale _returnvalue)) false false)))

(fn ConstructionScript)