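; BP_SideScrollGameMode is the game mode for a two-player local side-scrolling level with a shared camera.
; On BeginPlay it removes the default player, creates both players by switching DefaultPawnClass between the two side-scroll pawns, and disables splitscreen.
; It then points both controllers at the level's BP_Camera, runs its setup, offsets the characters to opposite Y positions, and triggers start spawning on BP_PlayerSpawning_Side.
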(event Custom|SpawnPlayers
  ;[1 1 1] This will spawn the default third person player, delete it and then spawn player 1 and player 2
  (Class|GameplayStatics|RemovePlayer (Game|GetPlayerController 0) true)
  (Variables|Default|SetDefaultPawnClass "/Game/GameBehaviour/Characters/Player/SideScroll/BP_Player1_SideScroll.BP_Player1_SideScroll_C")
  (Class|GameplayStatics|CreatePlayer 0)
  (Variables|Default|SetDefaultPawnClass "/Game/GameBehaviour/Characters/Player/SideScroll/BP_Player2_SideScroll.BP_Player2_SideScroll_C")
  (Class|GameplayStatics|CreatePlayer 1)
  (Class|GameplayStatics|SetForceDisableSplitscreen true))

(event EventBeginPlay
  (bind _returnvalue (Game|GetPlayerCharacter 0))
  (bind _returnvalue_2 (Game|GetPlayerCharacter 1))
  (bind _returnvalue_3 (Transformation|GetActorLocation _returnvalue_2))
  (bind _returnvalue_4 (Transformation|GetActorLocation _returnvalue))
  (bind _outactors (Actor|GetAllActorsOfClass "/Game/GameBehaviour/Core/Checkpoints/SideScroll/BP_PlayerSpawning_Side.BP_PlayerSpawning_Side_C"))
  (Variables|Default|SetPlayerSpawning (Utilities|Array|Get(acopy) _outactors))
  (CallFunction|SpawnPlayers)
  (bind _outactors_2 (Actor|GetAllActorsOfClass "/Game/GameBehaviour/Characters/Player/SideScroll/BP_Camera.BP_Camera_C"))
  (Variables|Default|SetCamera (Utilities|Array|Get(acopy) _outactors_2))
  (Game|Player|SetViewTargetwithBlend (Game|GetPlayerController 0) (Variables|Default|GetCamera) 0.0 "VTBlend_Linear" 0.0 false)
  (Game|Player|SetViewTargetwithBlend (Game|GetPlayerController 1) (Variables|Default|GetCamera) 0.0 "VTBlend_Linear" 0.0 false)
  (Default|CameraSetup (Variables|Default|GetCamera))
  (Transformation|SetActorLocation _returnvalue (Math|Vector|MakeVector (.x _returnvalue_4) 6e+01 (.z _returnvalue_4)) false false)
  (Transformation|SetActorLocation _returnvalue_2 (Math|Vector|MakeVector (.x _returnvalue_3) -6e+01 (.z _returnvalue_3)) false false)
  (Utilities|IsValid (Variables|Default|GetPlayerSpawning)
    (:Is%20Valid
      (Default|SetStartSpawn (Variables|Default|GetPlayerSpawning)))))

(fn ConstructionScript)