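; BP_PlayerSpawning handles start placement and respawning for two local players, BP_Player1 and BP_Player2.
; SetStartSpawn caches both player references, moves each to its start location and stores that as its spawn point.
; RespawnPlayer matches the dead player, disables its movement, waits briefly, moves it to its stored spawn point and restores walking.
; BeginPlay is empty, so SetStartSpawn is not called within this Blueprint.
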(event EventRespawnPlayer
  (params (DeadPlayer :type Actor%20Object%20Reference))
  ;[1 1 1] Checks to see which player was destroyed and respawns them accordingly
  (if (== DeadPlayer (Variables|Default|GetAs%20BP%20Player%201))
    (Pawn|Components|CharacterMovement|DisableMovement (Variables|/Script/Engine.Character|GetCharacterMovement (Variables|Default|GetAs%20BP%20Player%201)))
    (Utilities|FlowControl|Delay 0.3)
    (Transformation|SetActorLocation (Variables|Default|GetAs%20BP%20Player%201) (Variables|Default|GetPlayer1Spawn) false false)
    (Pawn|Components|CharacterMovement|SetMovementMode (Variables|/Script/Engine.Character|GetCharacterMovement (Variables|Default|GetAs%20BP%20Player%201)) "MOVE_Walking" 0)
    (elif (== DeadPlayer (Variables|Default|GetAs%20BP%20Player%202))
      (Pawn|Components|CharacterMovement|DisableMovement (Variables|/Script/Engine.Character|GetCharacterMovement (Variables|Default|GetAs%20BP%20Player%202)))
      (Utilities|FlowControl|Delay 0.3)
      (Transformation|SetActorLocation (Variables|Default|GetAs%20BP%20Player%202) (Variables|Default|GetPlayer2Spawn) false false)
      (Pawn|Components|CharacterMovement|SetMovementMode (Variables|/Script/Engine.Character|GetCharacterMovement (Variables|Default|GetAs%20BP%20Player%202)) "MOVE_Walking" 0))))

(event EventBeginPlay)

(fn ConstructionScript)

(fn SetStartSpawn
  (bind _player1start (Variables|Default|GetPlayer1Start))
  (bind _player2start (Variables|Default|GetPlayer2Start))
  (bind _asbp_player_1 (Utilities|Casting|CastToBP_Player1 (Game|GetPlayerCharacter 0)))
  (Variables|Default|SetAs%20BP%20Player%201 _asbp_player_1)
  (bind _asbp_player_2 (Utilities|Casting|CastToBP_Player2 (Game|GetPlayerCharacter 1)))
  (Variables|Default|SetAs%20BP%20Player%202 _asbp_player_2)
  (Transformation|SetActorLocation (Game|GetPlayerCharacter 0) _player1start false false)
  (Variables|Default|SetPlayer1Spawn _player1start)
  (Transformation|SetActorLocation (Game|GetPlayerCharacter 1) _player2start false false)
  (Variables|Default|SetPlayer2Spawn _player2start))