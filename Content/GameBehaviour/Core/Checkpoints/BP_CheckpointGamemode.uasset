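; BP_CheckpointGamemode is a game mode that respawns the player after their BP_Player1 character is destroyed.
; On BeginPlay it binds to the OnDestroyed event of the first player's character.
; When that fires, it waits briefly, spawns a new BP_Player1 at the SpawnLocation transform and has the player controller possess it.
; It then calls Respawn to bind the new pawn, so the cycle repeats; nothing here updates SpawnLocation.
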(event Custom|OnDestroyed_
  (params (DestroyedActor :type Actor%20Object%20Reference))
  (Utilities|FlowControl|Delay 2.0)
  (bind _returnvalue (Game|SpawnActorfromClass "/Game/GameBehaviour/Characters/Player/SplitScreen/BP_Player1.BP_Player1_C" (Variables|Default|GetSpawnLocation) "Undefined" 0 0))
  (Pawn|Possess (Game|GetPlayerController 0) _returnvalue)
  (CallFunction|Respawn))

(event Custom|Respawn
  (bind _asbp_player_1 (Utilities|Casting|CastToBP_Player1 (Game|GetPlayerCharacter 0)))
  (Game|BindEventtoOnDestroyed _asbp_player_1 (delegate Custom|OnDestroyed_)))

(event EventBeginPlay
  (bind _asbp_player_1 (Utilities|Casting|CastToBP_Player1 (Game|GetPlayerCharacter 0)))
  (Game|BindEventtoOnDestroyed _asbp_player_1 (delegate Custom|OnDestroyed_)))

(fn ConstructionScript)