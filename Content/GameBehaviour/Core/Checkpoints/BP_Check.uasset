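; BP_Check is a two-player checkpoint trigger that updates respawn points on the BP_PlayerSpawning actor found at BeginPlay.
; On box overlap, MultiSpawn mode lets any actor tagged Player set both spawns, while otherwise Player1 and Player2 tags each set only their own.
; Each spawn uses its configured respawn location, falling back to the checkpoint's location when that is zero.
; Boolean latches make each assignment happen only once per checkpoint.
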(event OnComponentBeginOverlap(Box)
  (params (OverlappedComponent :type Primitive%20Component%20Object%20Reference) (OtherActor :type Actor%20Object%20Reference) (OtherComp :type Primitive%20Component%20Object%20Reference) (OtherBodyIndex :type Integer) (bFromSweep :type Boolean) (SweepResult :type Hit%20Result%20Structure%20%28by%20ref%29))
  (if (Variables|Default|GetMultiSpawn?)
    ;[1 1 1] Set Both Players Spawns
    (if (Actor|ActorHasTag OtherActor "Player")
      (if (not (Variables|Default|GetplayersGot))
        (if (Utilities|Operators|EqualEqual :A (Variables|Default|GetPlayer1RespawnLocation))
          (Variables|/Game/GameBehaviour/Core/Checkpoints/BP_PlayerSpawning.BP_PlayerSpawning_C|SetPlayer1Spawn (Variables|Default|GetPlayerSpawning) (Transformation|GetActorLocation))
          (else
            (Variables|/Game/GameBehaviour/Core/Checkpoints/BP_PlayerSpawning.BP_PlayerSpawning_C|SetPlayer1Spawn (Variables|Default|GetPlayerSpawning) (Variables|Default|GetPlayer1RespawnLocation))))
        (if (Utilities|Operators|EqualEqual :A (Variables|Default|GetPlayer2RespawnLocation))
          (Variables|/Game/GameBehaviour/Core/Checkpoints/BP_PlayerSpawning.BP_PlayerSpawning_C|SetPlayer2Spawn (Variables|Default|GetPlayerSpawning) (Transformation|GetActorLocation))
          (else
            (Variables|/Game/GameBehaviour/Core/Checkpoints/BP_PlayerSpawning.BP_PlayerSpawning_C|SetPlayer2Spawn (Variables|Default|GetPlayerSpawning) (Variables|Default|GetPlayer2RespawnLocation))))
        (Variables|Default|SetplayersGot true)))
    (else
      ;[1 1 1] Set Player 1 Spawn
      (if (Actor|ActorHasTag OtherActor "Player1")
        (if (not (Variables|Default|Getplayer1got))
          (if (Utilities|Operators|EqualEqual :A (Variables|Default|GetPlayer1RespawnLocation))
            (Variables|/Game/GameBehaviour/Core/Checkpoints/BP_PlayerSpawning.BP_PlayerSpawning_C|SetPlayer1Spawn (Variables|Default|GetPlayerSpawning) (Transformation|GetActorLocation))
            (else
              (Variables|/Game/GameBehaviour/Core/Checkpoints/BP_PlayerSpawning.BP_PlayerSpawning_C|SetPlayer1Spawn (Variables|Default|GetPlayerSpawning) (Variables|Default|GetPlayer1RespawnLocation))))
          (Variables|Default|Setplayer1got true))
        (else
          ;[1 1 1] Set Player 2 Spawn
          (if (Actor|ActorHasTag OtherActor "Player2")
            (if (not (Variables|Default|Getplayer2got))
              (if (Utilities|Operators|EqualEqual :A (Variables|Default|GetPlayer2RespawnLocation))
                (Variables|/Game/GameBehaviour/Core/Checkpoints/BP_PlayerSpawning.BP_PlayerSpawning_C|SetPlayer2Spawn (Variables|Default|GetPlayerSpawning) (Transformation|GetActorLocation))
                (else
                  (Variables|/Game/GameBehaviour/Core/Checkpoints/BP_PlayerSpawning.BP_PlayerSpawning_C|SetPlayer2Spawn (Variables|Default|GetPlayerSpawning) (Variables|Default|GetPlayer2RespawnLocation))))
              (Variables|Default|Setplayer2got true))))))))

(event EventBeginPlay
  (bind _outactors (Actor|GetAllActorsOfClass "/Game/GameBehaviour/Core/Checkpoints/BP_PlayerSpawning.BP_PlayerSpawning_C"))
  (Variables|Default|SetPlayerSpawning (Utilities|Array|Get(acopy) _outactors)))

(fn ConstructionScript)