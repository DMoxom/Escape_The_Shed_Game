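; Side-scroll checkpoint actor that updates player respawn points when a player enters its box.
; On BeginPlay it finds the BP_PlayerSpawning_Side actor and writes spawn locations to it on overlap.
; With MultiSpawn, any Player-tagged actor updates both spawns; otherwise each player class updates only its own.
; Unset respawn overrides fall back to the checkpoint's location, with the per-player mode testing only X and Z for zero.
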(event OnComponentBeginOverlap(Box)
  (params (OverlappedComponent :type Primitive%20Component%20Object%20Reference) (OtherActor :type Actor%20Object%20Reference) (OtherComp :type Primitive%20Component%20Object%20Reference) (OtherBodyIndex :type Integer) (bFromSweep :type Boolean) (SweepResult :type Hit%20Result%20Structure%20%28by%20ref%29))
  (bind _player2respawnlocation (Variables|Default|GetPlayer2RespawnLocation))
  (bind _player1respawnlocation (Variables|Default|GetPlayer1RespawnLocation))
  (if (Variables|Default|GetMultiSpawn?)
    (if (Actor|ActorHasTag OtherActor "Player")
      (if (Utilities|Operators|EqualEqual :A (Variables|Default|GetPlayer1RespawnLocation))
        (Variables|/Game/GameBehaviour/Core/Checkpoints/SideScroll/BP_PlayerSpawning_Side.BP_PlayerSpawning_Side_C|SetPlayer1Spawn (Variables|Default|GetPlayerSpawning2) (Transformation|GetActorLocation))
        (else
          (Variables|/Game/GameBehaviour/Core/Checkpoints/SideScroll/BP_PlayerSpawning_Side.BP_PlayerSpawning_Side_C|SetPlayer1Spawn (Variables|Default|GetPlayerSpawning2) (Variables|Default|GetPlayer1RespawnLocation))))
      (if (Utilities|Operators|EqualEqual :A (Variables|Default|GetPlayer2RespawnLocation))
        (Variables|/Game/GameBehaviour/Core/Checkpoints/SideScroll/BP_PlayerSpawning_Side.BP_PlayerSpawning_Side_C|SetPlayer2Spawn (Variables|Default|GetPlayerSpawning2) (Transformation|GetActorLocation))
        (else
          (Variables|/Game/GameBehaviour/Core/Checkpoints/SideScroll/BP_PlayerSpawning_Side.BP_PlayerSpawning_Side_C|SetPlayer2Spawn (Variables|Default|GetPlayerSpawning2) (Variables|Default|GetPlayer2RespawnLocation)))))
    (else
      (Utilities|Casting|CastToBP_Player1_SideScroll OtherActor
        (:then
          (if (and (== (.x _player1respawnlocation) 0.0) (== (.z _player1respawnlocation) 0.0))
            (Variables|/Game/GameBehaviour/Core/Checkpoints/SideScroll/BP_PlayerSpawning_Side.BP_PlayerSpawning_Side_C|SetPlayer1Spawn (Variables|Default|GetPlayerSpawning2) (Transformation|GetActorLocation))
            (else
              (Variables|/Game/GameBehaviour/Core/Checkpoints/SideScroll/BP_PlayerSpawning_Side.BP_PlayerSpawning_Side_C|SetPlayer1Spawn (Variables|Default|GetPlayerSpawning2) (Variables|Default|GetPlayer1RespawnLocation)))))
        (:CastFailed
          (Utilities|Casting|CastToBP_Player2_SideScroll OtherActor)
          (if (and (== (.x _player2respawnlocation) 0.0) (== (.z _player2respawnlocation) 0.0))
            (Variables|/Game/GameBehaviour/Core/Checkpoints/SideScroll/BP_PlayerSpawning_Side.BP_PlayerSpawning_Side_C|SetPlayer2Spawn (Variables|Default|GetPlayerSpawning2) (Transformation|GetActorLocation))
            (else
              (Variables|/Game/GameBehaviour/Core/Checkpoints/SideScroll/BP_PlayerSpawning_Side.BP_PlayerSpawning_Side_C|SetPlayer2Spawn (Variables|Default|GetPlayerSpawning2) (Variables|Default|GetPlayer2RespawnLocation)))))))))

(event EventBeginPlay
  (bind _outactors (Actor|GetAllActorsOfClass "/Game/GameBehaviour/Core/Checkpoints/SideScroll/BP_PlayerSpawning_Side.BP_PlayerSpawning_Side_C"))
  (Variables|Default|SetPlayerSpawning2 (Utilities|Array|Get(acopy) _outactors)))

(fn ConstructionScript)