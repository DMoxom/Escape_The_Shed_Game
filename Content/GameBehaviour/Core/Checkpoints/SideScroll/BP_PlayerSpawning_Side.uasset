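; Respawn manager for the two players in side-scroll gameplay.
; SetStartSpawn caches both side-scroll characters and records their current locations as spawn points.
; RespawnPlayer matches the dead player, disables its movement, then after a short delay moves it to its spawn's X and Z and restores walking.
; Y is fixed on opposite sides of zero, giving each player a separate depth lane.
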(event EventRespawnPlayer
  (params (DeadPlayer :type Actor%20Object%20Reference))
  (bind _player1spawn (Variables|Default|GetPlayer1Spawn))
  (bind _player2spawn (Variables|Default|GetPlayer2Spawn))
  ;[1 1 1] Checks to see which player was destroyed and respawns them accordingly
  (if (== DeadPlayer (Variables|Default|GetAs%20BP%20Player%201%20Side%20Scroll))
    (Pawn|Components|CharacterMovement|DisableMovement (Variables|/Script/Engine.Character|GetCharacterMovement (Variables|Default|GetAs%20BP%20Player%201%20Side%20Scroll)))
    (Utilities|FlowControl|Delay 0.3)
    (Transformation|SetActorLocation (Variables|Default|GetAs%20BP%20Player%201%20Side%20Scroll) (Math|Vector|MakeVector (.x _player1spawn) 6e+01 (.z _player1spawn)) false false)
    (Pawn|Components|CharacterMovement|SetMovementMode (Variables|/Script/Engine.Character|GetCharacterMovement (Variables|Default|GetAs%20BP%20Player%201%20Side%20Scroll)) "MOVE_Walking" 0)
    (elif (== DeadPlayer (Variables|Default|GetAs%20BP%20Player%202%20Side%20Scroll))
      (Pawn|Components|CharacterMovement|DisableMovement (Variables|/Script/Engine.Character|GetCharacterMovement (Variables|Default|GetAs%20BP%20Player%202%20Side%20Scroll)))
      (Utilities|FlowControl|Delay 0.3)
      (Transformation|SetActorLocation (Variables|Default|GetAs%20BP%20Player%202%20Side%20Scroll) (Math|Vector|MakeVector (.x _player2spawn) -6e+01 (.z _player2spawn)) false false)
      (Pawn|Components|CharacterMovement|SetMovementMode (Variables|/Script/Engine.Character|GetCharacterMovement (Variables|Default|GetAs%20BP%20Player%202%20Side%20Scroll)) "MOVE_Walking" 0))))

(fn ConstructionScript)

(fn SetStartSpawn
  (bind _asbp_player_1_side_scroll (Utilities|Casting|CastToBP_Player1_SideScroll (Game|GetPlayerCharacter 0)))
  (Variables|Default|SetAs%20BP%20Player%201%20Side%20Scroll _asbp_player_1_side_scroll)
  (bind _asbp_player_2_side_scroll (Utilities|Casting|CastToBP_Player2_SideScroll (Game|GetPlayerCharacter 1)))
  (Variables|Default|SetAs%20BP%20Player%202%20Side%20Scroll _asbp_player_2_side_scroll)
  (Variables|Default|SetPlayer1Spawn (Transformation|GetActorLocation (Game|GetPlayerCharacter 0)))
  (Variables|Default|SetPlayer2Spawn (Transformation|GetActorLocation (Game|GetPlayerCharacter 1))))