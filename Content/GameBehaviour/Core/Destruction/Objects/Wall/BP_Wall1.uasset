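; Wall object that can be destroyed and repaired, toggling which action Player 1 (repair) and Player 2 (destroy) are allowed while it is selected.
; Twenty fragment meshes receive a shared Pivot material vector at BeginPlay, which also flags the wall as destroyed.
; One timeline drives two staged material alphas on every fragment, playing forward to destruct and reversing to repair.
; Highlighting renders fragments to custom depth while selected.
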(event EventBeginPlay
  (bind _box_geometrycollection_sm_1_ (Variables|Default|GetBox_GeometryCollection_SM_1_))
  (bind _output_get (Variables|Default|SetDestruction%20Fragments (Utilities|Array|MakeArray _box_geometrycollection_sm_1_ (Variables|Default|GetBox_GeometryCollection_SM_2_) (Variables|Default|GetBox_GeometryCollection_SM_3_) (Variables|Default|GetBox_GeometryCollection_SM_4_) (Variables|Default|GetBox_GeometryCollection_SM_5_) (Variables|Default|GetBox_GeometryCollection_SM_6_) (Variables|Default|GetBox_GeometryCollection_SM_7_) (Variables|Default|GetBox_GeometryCollection_SM_8_) (Variables|Default|GetBox_GeometryCollection_SM_9_) (Variables|Default|GetBox_GeometryCollection_SM_10_) (Variables|Default|GetBox_GeometryCollection_SM_11_) (Variables|Default|GetBox_GeometryCollection_SM_12_) (Variables|Default|GetBox_GeometryCollection_SM_13_) (Variables|Default|GetBox_GeometryCollection_SM_14_) (Variables|Default|GetBox_GeometryCollection_SM_15_) (Variables|Default|GetBox_GeometryCollection_SM_16_) (Variables|Default|GetBox_GeometryCollection_SM_17_) (Variables|Default|GetBox_GeometryCollection_SM_18_) (Variables|Default|GetBox_GeometryCollection_SM_19_) (Variables|Default|GetBox_GeometryCollection_SM_20_))))
  (for _array_element _output_get
    (Rendering|Material|SetVectorParameterValueonMaterials _array_element "Pivot" (Transformation|GetWorldLocation _box_geometrycollection_sm_1_))
    (Utilities|FlowControl|Delay 0.2)
    (bind _asbp_player_1 (Utilities|Casting|CastToBP_Player1 (Game|GetPlayerCharacter 0)))
    (Variables|Default|SetAs%20BP%20Player%201 _asbp_player_1)
    (bind _asbp_player_2 (Utilities|Casting|CastToBP_Player2 (Game|GetPlayerCharacter 1)))
    (Variables|Default|SetAs%20BP%20Player%202 _asbp_player_2)
    (Variables|Default|SetIsDestroyed true)))

(event EventObjectHighlight
  (params (CanBeInteractedWith :type Boolean))
  (if CanBeInteractedWith
    (if (Variables|Default|GetIsSelectedLocal)
      (for _array_element (Variables|Default|GetDestruction%20Fragments)
        (Rendering|SetRenderCustomDepth _array_element true)))))

(event EventSelectObject
  (Variables|Default|SetIsSelectedLocal true)
  (if (Variables|Default|GetIsDestroyed)
    (Variables|/Game/GameBehaviour/Characters/Player/SplitScreen/BP_Player1.BP_Player1_C|SetCanBeRepaired (Variables|Default|GetAs%20BP%20Player%201) true)
    (Variables|/Game/GameBehaviour/Characters/Player/SplitScreen/BP_Player2.BP_Player2_C|SetCanBeDestroyed (Variables|Default|GetAs%20BP%20Player%202) false)
    (else
      (Variables|/Game/GameBehaviour/Characters/Player/SplitScreen/BP_Player1.BP_Player1_C|SetCanBeRepaired (Variables|Default|GetAs%20BP%20Player%201) false)
      (Variables|/Game/GameBehaviour/Characters/Player/SplitScreen/BP_Player2.BP_Player2_C|SetCanBeDestroyed (Variables|Default|GetAs%20BP%20Player%202) true))))

(event EventRepairObject
  (params (isRepairable :type Boolean))
  (if true
    (Variables|/Game/GameBehaviour/Characters/Player/SplitScreen/BP_Player1.BP_Player1_C|SetCanBeRepaired (Variables|Default|GetAs%20BP%20Player%201) false)
    (Variables|/Game/GameBehaviour/Characters/Player/SplitScreen/BP_Player2.BP_Player2_C|SetCanBeDestroyed (Variables|Default|GetAs%20BP%20Player%202) true)
    (Variables|Default|SetIsDestroyed false)
    (bind _newtrack_0 (Timeline|Destruction%20Reverse Reverse)
      (:Update
        (for _array_element (Variables|Default|GetDestruction%20Fragments)
          (Rendering|Material|SetScalarParameterValueonMaterials _array_element "Alpha 1" (Math|Float|Clamp(Float) (* _newtrack_0 2.0)))
          (Rendering|Material|SetScalarParameterValueonMaterials _array_element "Alpha 2" (Math|Float|Clamp(Float) (- (* _newtrack_0 2.0) 1.0))))))))

(event EventDeselectObject
  (Variables|Default|SetIsSelectedLocal false)
  (for _array_element (Variables|Default|GetDestruction%20Fragments)
    (Rendering|SetRenderCustomDepth _array_element false)))

(event EventDestructObject
  (params (isDestructable :type Boolean))
  (if true
    (Variables|/Game/GameBehaviour/Characters/Player/SplitScreen/BP_Player1.BP_Player1_C|SetCanBeRepaired (Variables|Default|GetAs%20BP%20Player%201) true)
    (Variables|/Game/GameBehaviour/Characters/Player/SplitScreen/BP_Player2.BP_Player2_C|SetCanBeDestroyed (Variables|Default|GetAs%20BP%20Player%202) false)
    (Variables|Default|SetIsDestroyed true)
    (bind _newtrack_0 (Timeline|Destruction%20Reverse Play)
      (:Update
        (for _array_element (Variables|Default|GetDestruction%20Fragments)
          (Rendering|Material|SetScalarParameterValueonMaterials _array_element "Alpha 1" (Math|Float|Clamp(Float) (* _newtrack_0 2.0)))
          (Rendering|Material|SetScalarParameterValueonMaterials _array_element "Alpha 2" (Math|Float|Clamp(Float) (- (* _newtrack_0 2.0) 1.0))))))))

(fn ConstructionScript)

(fn IsSelected
  (return false))