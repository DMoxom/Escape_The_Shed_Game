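; Side-scroller wheely bin that starts destroyed; Player 1 can repair it and Player 2 can destroy it again.
; Overlapping the highlight radius registers the bin with that player, while Tick toggles a custom-depth outline, stencil-coded for repair or destroy.
; A timeline plays or reverses a material alpha on the pivot-aware fragments, enabling collision only at zero.
; The equally toggled KillBox asks the spawner to respawn players it touches.
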(event OnComponentBeginOverlap(HighlightRadius)
  (params (OverlappedComponent :type Primitive%20Component%20Object%20Reference) (OtherActor :type Actor%20Object%20Reference) (OtherComp :type Primitive%20Component%20Object%20Reference) (OtherBodyIndex :type Integer) (bFromSweep :type Boolean) (SweepResult :type Hit%20Result%20Structure%20%28by%20ref%29))
  (bind _as_bp_player_1_side_scroll (Variables|Default|GetAs%20BP%20Player%201%20Side%20Scroll))
  (bind _as_bp_player_2_side_scroll (Variables|Default|GetAs%20BP%20Player%202%20Side%20Scroll))
  (Utilities|Casting|CastToBP_Player1_SideScroll OtherActor
    (:then
      (Variables|Default|SetisPlayer1Overlapping true)
      (Variables|/Game/GameBehaviour/Characters/Player/SideScroll/BP_Player1_SideScroll.BP_Player1_SideScroll_C|SetrepairingObject _as_bp_player_1_side_scroll self)
      (if (Variables|Default|GetIsDestroyed)
        (CallFunction|RepairedHighlight)
        (Variables|/Game/GameBehaviour/Characters/Player/SideScroll/BP_Player1_SideScroll.BP_Player1_SideScroll_C|SetcanRepair _as_bp_player_1_side_scroll true)
        (Variables|/Game/GameBehaviour/Characters/Player/SideScroll/BP_Player2_SideScroll.BP_Player2_SideScroll_C|SetcanDestroy (Variables|Default|GetAs%20BP%20Player%202%20Side%20Scroll) false)))
    (:CastFailed
      (Utilities|Casting|CastToBP_Player2_SideScroll OtherActor)
      (Variables|Default|SetisPlayer2Overlapping true)
      (Variables|/Game/GameBehaviour/Characters/Player/SideScroll/BP_Player2_SideScroll.BP_Player2_SideScroll_C|SetrepairingObject _as_bp_player_2_side_scroll self)
      (if (not (Variables|Default|GetIsDestroyed))
        (CallFunction|DestroyedHighlight)
        (Variables|/Game/GameBehaviour/Characters/Player/SideScroll/BP_Player1_SideScroll.BP_Player1_SideScroll_C|SetcanRepair (Variables|Default|GetAs%20BP%20Player%201%20Side%20Scroll) false)
        (Variables|/Game/GameBehaviour/Characters/Player/SideScroll/BP_Player2_SideScroll.BP_Player2_SideScroll_C|SetcanDestroy _as_bp_player_2_side_scroll true)))))

(event OnComponentEndOverlap(HighlightRadius)
  (params (OverlappedComponent :type Primitive%20Component%20Object%20Reference) (OtherActor :type Actor%20Object%20Reference) (OtherComp :type Primitive%20Component%20Object%20Reference) (OtherBodyIndex :type Integer))
  (bind _as_bp_player_2_side_scroll (Variables|Default|GetAs%20BP%20Player%202%20Side%20Scroll))
  (bind _as_bp_player_1_side_scroll (Variables|Default|GetAs%20BP%20Player%201%20Side%20Scroll))
  (Utilities|Casting|CastToBP_Player1_SideScroll OtherActor
    (:then
      (Variables|Default|SetisPlayer1Overlapping false)
      (Variables|/Game/GameBehaviour/Characters/Player/SideScroll/BP_Player1_SideScroll.BP_Player1_SideScroll_C|SetcanRepair _as_bp_player_1_side_scroll false)
      (Variables|/Game/GameBehaviour/Characters/Player/SideScroll/BP_Player1_SideScroll.BP_Player1_SideScroll_C|SetrepairingObject _as_bp_player_1_side_scroll 0))
    (:CastFailed
      (Utilities|Casting|CastToBP_Player2_SideScroll OtherActor)
      (Variables|Default|SetisPlayer2Overlapping false)
      (Variables|/Game/GameBehaviour/Characters/Player/SideScroll/BP_Player2_SideScroll.BP_Player2_SideScroll_C|SetcanDestroy _as_bp_player_2_side_scroll false)
      (Variables|/Game/GameBehaviour/Characters/Player/SideScroll/BP_Player2_SideScroll.BP_Player2_SideScroll_C|SetrepairingObject _as_bp_player_2_side_scroll 0))))

(event OnComponentBeginOverlap(KillBox)
  (params (OverlappedComponent :type Primitive%20Component%20Object%20Reference) (OtherActor :type Actor%20Object%20Reference) (OtherComp :type Primitive%20Component%20Object%20Reference) (OtherBodyIndex :type Integer) (bFromSweep :type Boolean) (SweepResult :type Hit%20Result%20Structure%20%28by%20ref%29))
  (if (Actor|ActorHasTag OtherActor "Player")
    (Class|BIPlayerDeath|RespawnPlayer(Message) (Variables|Default|GetPlayerSpawning) OtherActor)))

(event EventBeginPlay
  (bind _sm_wheely_bin_18_ (Variables|Default|GetSM_Wheely_bin_18_))
  (bind _output_get (Variables|Default|SetDestruction%20Fragments (Utilities|Array|MakeArray _sm_wheely_bin_18_ (Variables|Default|GetSM_Wheely_bin_19_) (Variables|Default|GetSM_Wheely_bin_1_) (Variables|Default|GetSM_Wheely_bin_20_) (Variables|Default|GetSM_Wheely_bin_21_) (Variables|Default|GetSM_Wheely_bin_22_) (Variables|Default|GetSM_Wheely_bin_23_) (Variables|Default|GetSM_Wheely_bin_10_) (Variables|Default|GetSM_Wheely_bin_11_) (Variables|Default|GetSM_Wheely_bin_12_) (Variables|Default|GetSM_Wheely_bin_13_) (Variables|Default|GetSM_Wheely_bin_17_) (Variables|Default|GetSM_Wheely_bin_14_) (Variables|Default|GetSM_Wheely_bin_15_) (Variables|Default|GetSM_Wheely_bin_16_) (Variables|Default|GetSM_Wheely_bin_24_) (Variables|Default|GetSM_Wheely_bin_4_) (Variables|Default|GetSM_Wheely_bin_5_) (Variables|Default|GetSM_Wheely_bin_6_) (Variables|Default|GetSM_Wheely_bin_3_) (Variables|Default|GetSM_Wheely_bin_7_) (Variables|Default|GetSM_Wheely_bin_8_) (Variables|Default|GetSM_Wheely_bin_9_) (Variables|Default|GetSM_Wheely_bin_26_) (Variables|Default|GetSM_Wheely_bin_27_) (Variables|Default|GetSM_Wheely_bin_28_) (Variables|Default|GetSM_Wheely_bin_25_) (Variables|Default|GetSM_Wheely_bin_29_) (Variables|Default|GetSM_Wheely_bin_2_) (Variables|Default|GetSM_Wheely_bin_30_) (Variables|Default|GetSM_Wheely_bin_31_))))
  (for _array_element _output_get
    (Rendering|Material|SetVectorParameterValueonMaterials _array_element "Pivot" (Transformation|GetWorldLocation _sm_wheely_bin_18_))
    (Utilities|FlowControl|Delay 0.2)
    (bind _asbp_player_1_side_scroll (Utilities|Casting|CastToBP_Player1_SideScroll (Game|GetPlayerCharacter 0)))
    (Variables|Default|SetAs%20BP%20Player%201%20Side%20Scroll _asbp_player_1_side_scroll)
    (bind _asbp_player_2_side_scroll (Utilities|Casting|CastToBP_Player2_SideScroll (Game|GetPlayerCharacter 1)))
    (Variables|Default|SetAs%20BP%20Player%202%20Side%20Scroll _asbp_player_2_side_scroll)
    (Variables|Default|SetIsDestroyed true)
    (bind _outactors (Actor|GetAllActorsOfClass "/Game/GameBehaviour/Core/Checkpoints/SideScroll/BP_PlayerSpawning_Side.BP_PlayerSpawning_Side_C"))
    (Variables|Default|SetPlayerSpawning (Utilities|Array|Get(acopy) _outactors))
    (Collision|SetCollisionEnabled (Variables|Default|GetKillBox) "NoCollision")
    (for _array_element_2 (Variables|Default|GetDestruction%20Fragments)
      (Collision|SetCollisionEnabled _array_element_2 "NoCollision")
      (Rendering|SetCustomDepthStencilValue _array_element_2 (Variables|Default|GetRepairHiglight)))))

(event EventObjectHighlight
  (params (CanBeInteractedWith :type Boolean))
  (if CanBeInteractedWith
    (for _array_element (Variables|Default|GetDestruction%20Fragments)
      (Rendering|SetRenderCustomDepth _array_element true))))

(event EventSelectObject)

(event EventRepairObject
  (params (isRepairable :type Boolean))
  (if true
    (Variables|/Game/GameBehaviour/Characters/Player/SideScroll/BP_Player1_SideScroll.BP_Player1_SideScroll_C|SetcanRepair (Variables|Default|GetAs%20BP%20Player%201%20Side%20Scroll) false)
    (Variables|/Game/GameBehaviour/Characters/Player/SideScroll/BP_Player2_SideScroll.BP_Player2_SideScroll_C|SetcanDestroy (Variables|Default|GetAs%20BP%20Player%202%20Side%20Scroll) true)
    (Variables|Default|SetIsDestroyed false)
    (CallFunction|DestroyedHighlight)
    (bind _newtrack_0 (Timeline|Timeline Play)
      (:Update
        (for _array_element (Variables|Default|GetDestruction%20Fragments)
          (Rendering|Material|SetScalarParameterValueonMaterials _array_element "Alpha 2" _newtrack_0)
          (if (== _newtrack_0 0.0)
            (Collision|SetCollisionEnabled (Variables|Default|GetKillBox) "QueryAndPhysics")
            (for _array_element_2 (Variables|Default|GetDestruction%20Fragments)
              (Collision|SetCollisionEnabled _array_element_2 "QueryAndPhysics"))
            (else
              (Collision|SetCollisionEnabled (Variables|Default|GetKillBox) "NoCollision")
              (for _array_element_3 (Variables|Default|GetDestruction%20Fragments)
                (Collision|SetCollisionEnabled _array_element_3 "NoCollision")))))))))

(event EventDeselectObject
  (Variables|Default|SetIsSelectedLocal false)
  (for _array_element (Variables|Default|GetDestruction%20Fragments)
    (Rendering|SetRenderCustomDepth _array_element false)))

(event EventDestructObject
  (params (isDestructable :type Boolean))
  (if true
    (Variables|/Game/GameBehaviour/Characters/Player/SideScroll/BP_Player1_SideScroll.BP_Player1_SideScroll_C|SetcanRepair (Variables|Default|GetAs%20BP%20Player%201%20Side%20Scroll) true)
    (Variables|/Game/GameBehaviour/Characters/Player/SideScroll/BP_Player2_SideScroll.BP_Player2_SideScroll_C|SetcanDestroy (Variables|Default|GetAs%20BP%20Player%202%20Side%20Scroll) false)
    (Variables|Default|SetIsDestroyed true)
    (CallFunction|RepairedHighlight)
    (bind _newtrack_0 (Timeline|Timeline Reverse)
      (:Update
        (for _array_element (Variables|Default|GetDestruction%20Fragments)
          (Rendering|Material|SetScalarParameterValueonMaterials _array_element "Alpha 2" _newtrack_0)
          (if (== _newtrack_0 0.0)
            (Collision|SetCollisionEnabled (Variables|Default|GetKillBox) "QueryAndPhysics")
            (for _array_element_2 (Variables|Default|GetDestruction%20Fragments)
              (Collision|SetCollisionEnabled _array_element_2 "QueryAndPhysics"))
            (else
              (Collision|SetCollisionEnabled (Variables|Default|GetKillBox) "NoCollision")
              (for _array_element_3 (Variables|Default|GetDestruction%20Fragments)
                (Collision|SetCollisionEnabled _array_element_3 "NoCollision")))))))))

(event EventTick
  (params (DeltaSeconds :type Float%20%28single-precision%29))
  (if (Variables|Default|GetisPlayer1Overlapping)
    (if (Variables|Default|GetIsDestroyed)
      (CallFunction|ObjectHighlight true :!label _label)
      (elif (Variables|Default|GetisPlayer2Overlapping)
        (goto _label)
        (else
          (CallFunction|DeselectObject))))
    (elif (Variables|Default|GetisPlayer2Overlapping)
      (if (Variables|Default|GetIsDestroyed)
        (if (Variables|Default|GetisPlayer1Overlapping)
          (CallFunction|ObjectHighlight true :!label _label_2)
          (else
            (CallFunction|DeselectObject)))
        (else
          (goto _label_2)))
      (else
        (CallFunction|DeselectObject)))))

(fn ConstructionScript)

(fn RepairedHighlight
  (for _array_element (Variables|Default|GetDestruction%20Fragments)
    (Rendering|SetCustomDepthStencilValue _array_element (Variables|Default|GetRepairHiglight))))

(fn DestroyedHighlight
  (for _array_element (Variables|Default|GetDestruction%20Fragments)
    (Rendering|SetCustomDepthStencilValue _array_element (Variables|Default|GetDestroyHiglight))))

(fn IsSelected
  (return false))