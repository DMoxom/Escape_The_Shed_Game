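; Destructible box prop that Player 2 can destroy and Player 1 can repair, with selection and state updating each player's ability flags.
; A timeline drives a material alpha across 33 fragment meshes around a shared pivot, playing forward to destroy and reversing to repair.
; Lid and body collision is off unless the timeline value is zero.
; Custom depth highlights the selected box, with stencil values distinguishing destroy from repair.
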(event EventBeginPlay
  (bind _sm_container_low_with_lid_geometrycollection_1_ (Variables|Default|GetSM_Container_Low_With_Lid_GeometryCollection_1_))
  (bind _output_get (Variables|Default|SetDestruction%20Fragments (Utilities|Array|MakeArray _sm_container_low_with_lid_geometrycollection_1_ (Variables|Default|GetSM_Container_Low_With_Lid_GeometryCollection_2_) (Variables|Default|GetSM_Container_Low_With_Lid_GeometryCollection_3_) (Variables|Default|GetSM_Container_Low_With_Lid_GeometryCollection_4_) (Variables|Default|GetSM_Container_Low_With_Lid_GeometryCollection_5_) (Variables|Default|GetSM_Container_Low_With_Lid_GeometryCollection_6_) (Variables|Default|GetSM_Container_Low_With_Lid_GeometryCollection_7_) (Variables|Default|GetSM_Container_Low_With_Lid_GeometryCollection_8_) (Variables|Default|GetSM_Container_Low_With_Lid_GeometryCollection_9_) (Variables|Default|GetSM_Container_Low_With_Lid_GeometryCollection_10_) (Variables|Default|GetSM_Container_Low_With_Lid_GeometryCollection_11_) (Variables|Default|GetSM_Container_Low_With_Lid_GeometryCollection_12_) (Variables|Default|GetSM_Container_Low_With_Lid_GeometryCollection_13_) (Variables|Default|GetSM_Container_Low_With_Lid_GeometryCollection_14_) (Variables|Default|GetSM_Container_Low_With_Lid_GeometryCollection_15_) (Variables|Default|GetSM_Container_Low_With_Lid_GeometryCollection_16_) (Variables|Default|GetSM_Container_Low_With_Lid_GeometryCollection_17_) (Variables|Default|GetSM_Container_Low_With_Lid_GeometryCollection_18_) (Variables|Default|GetSM_Container_Low_With_Lid_GeometryCollection_19_) (Variables|Default|GetSM_Container_Low_With_Lid_GeometryCollection_20_) (Variables|Default|GetSM_Container_Low_With_Lid_GeometryCollection_21_) (Variables|Default|GetSM_Container_Low_With_Lid_GeometryCollection_22_) (Variables|Default|GetSM_Container_Low_With_Lid_GeometryCollection_23_) (Variables|Default|GetSM_Container_Low_With_Lid_GeometryCollection_24_) (Variables|Default|GetSM_Container_Low_With_Lid_GeometryCollection_25_) (Variables|Default|GetSM_Container_Low_With_Lid_GeometryCollection_26_) (Variables|Default|GetSM_Container_Low_With_Lid_GeometryCollection_27_) (Variables|Default|GetSM_Container_Low_With_Lid_GeometryCollection_28_) (Variables|Default|GetSM_Container_Low_With_Lid_GeometryCollection_29_) (Variables|Default|GetSM_Container_Low_With_Lid_GeometryCollection_30_) (Variables|Default|GetSM_Container_Low_With_Lid_GeometryCollection_31_) (Variables|Default|GetSM_Container_Low_With_Lid_GeometryCollection_32_) (Variables|Default|GetSM_Container_Low_With_Lid_GeometryCollection_33_))))
  (for _array_element _output_get
    (Rendering|Material|SetVectorParameterValueonMaterials _array_element "Pivot" (Transformation|GetWorldLocation _sm_container_low_with_lid_geometrycollection_1_))
    (Utilities|FlowControl|Delay 0.2)
    (bind _asbp_player_1 (Utilities|Casting|CastToBP_Player1 (Game|GetPlayerCharacter 0)))
    (Variables|Default|SetAs%20BP%20Player%201 _asbp_player_1)
    (bind _asbp_player_2 (Utilities|Casting|CastToBP_Player2 (Game|GetPlayerCharacter 1)))
    (Variables|Default|SetAs%20BP%20Player%202 _asbp_player_2)
    (Variables|Default|SetIsDestroyed false)
    (Collision|SetCollisionEnabled (Variables|Default|GetBox_Lid) "QueryAndPhysics")
    (for _array_element_2 (Variables|Default|GetDestruction%20Fragments)
      (Rendering|SetCustomDepthStencilValue _array_element_2 (Variables|Default|GetDestroyHiglight)))))

(event EventObjectHighlight
  (params (CanBeInteractedWith :type Boolean))
  (if CanBeInteractedWith
    (if (Variables|Default|GetIsSelectedLocal)
      (for _array_element (Variables|Default|GetDestruction%20Fragments)
        (Rendering|SetRenderCustomDepth _array_element true)))))

(event EventSelectObject
  (Variables|Default|SetIsSelectedLocal true)
  (if (Variables|Default|GetIsDestroyed)
    (Variables|/Game/GameBehaviour/Characters/Player/SplitScreen/BP_Player1.BP_Player1_C|SetCanBeRepaired (Variables|Default|GetAs%20BP%20Player%201) true)
    (Variables|/Game/GameBehaviour/Characters/Player/SplitScreen/BP_Player2.BP_Player2_C|SetCanBeDestroyed (Variables|Default|GetAs%20BP%20Player%202) false)
    (else
      (Variables|/Game/GameBehaviour/Characters/Player/SplitScreen/BP_Player1.BP_Player1_C|SetCanBeRepaired (Variables|Default|GetAs%20BP%20Player%201) false)
      (Variables|/Game/GameBehaviour/Characters/Player/SplitScreen/BP_Player2.BP_Player2_C|SetCanBeDestroyed (Variables|Default|GetAs%20BP%20Player%202) true))))

(event EventRepairObject
  (params (isRepairable :type Boolean))
  (bind _box_lid (Variables|Default|GetBox_Lid))
  (if true
    (Variables|/Game/GameBehaviour/Characters/Player/SplitScreen/BP_Player1.BP_Player1_C|SetCanBeRepaired (Variables|Default|GetAs%20BP%20Player%201) false)
    (Variables|/Game/GameBehaviour/Characters/Player/SplitScreen/BP_Player2.BP_Player2_C|SetCanBeDestroyed (Variables|Default|GetAs%20BP%20Player%202) true)
    (Variables|Default|SetIsDestroyed false)
    (CallFunction|DestroyedHighlight)
    (bind _newtrack_0 (Timeline|Destruction Reverse)
      (:Update
        (for _array_element (Variables|Default|GetDestruction%20Fragments)
          (Rendering|Material|SetScalarParameterValueonMaterials _array_element "Alpha 2" _newtrack_0)
          (if (== _newtrack_0 0.0)
            (Collision|SetCollisionEnabled _box_lid "QueryAndPhysics")
            (else
              (Collision|SetCollisionEnabled _box_lid "NoCollision"))))))))

(event EventDeselectObject
  (Variables|Default|SetIsSelectedLocal false)
  (for _array_element (Variables|Default|GetDestruction%20Fragments)
    (Rendering|SetRenderCustomDepth _array_element false)))

(event EventDestructObject
  (params (isDestructable :type Boolean))
  (bind _box_lid (Variables|Default|GetBox_Lid))
  (if true
    (Variables|/Game/GameBehaviour/Characters/Player/SplitScreen/BP_Player1.BP_Player1_C|SetCanBeRepaired (Variables|Default|GetAs%20BP%20Player%201) true)
    (Variables|/Game/GameBehaviour/Characters/Player/SplitScreen/BP_Player2.BP_Player2_C|SetCanBeDestroyed (Variables|Default|GetAs%20BP%20Player%202) false)
    (Variables|Default|SetIsDestroyed true)
    (CallFunction|RepairedHighlight)
    (bind _newtrack_0 (Timeline|Destruction Play)
      (:Update
        (for _array_element (Variables|Default|GetDestruction%20Fragments)
          (Rendering|Material|SetScalarParameterValueonMaterials _array_element "Alpha 2" _newtrack_0)
          (if (== _newtrack_0 0.0)
            (Collision|SetCollisionEnabled _box_lid "QueryAndPhysics")
            (else
              (Collision|SetCollisionEnabled _box_lid "NoCollision"))))))))

(fn ConstructionScript)

(fn RepairedHighlight
  (for _array_element (Variables|Default|GetDestruction%20Fragments)
    (Rendering|SetCustomDepthStencilValue _array_element (Variables|Default|GetRepairHiglight))))

(fn DestroyedHighlight
  (for _array_element (Variables|Default|GetDestruction%20Fragments)
    (Rendering|SetCustomDepthStencilValue _array_element (Variables|Default|GetDestroyHiglight))))

(fn IsSelected
  (return false))