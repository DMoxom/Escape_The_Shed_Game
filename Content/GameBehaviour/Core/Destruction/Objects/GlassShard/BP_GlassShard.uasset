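; Destructible glass shard for two-player play, which Player 2 can destroy and Player 1 can repair.
; Selection sets each player's ability flag and allows a custom-depth highlight, with stencil values distinguishing repair from destroy.
; Destroying and repairing play a timeline forward or back, driving a pivot-based material parameter on seventeen fragment meshes and toggling collision.
; KillBox and respawn logic is present but unconnected.
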(event EventBeginPlay
  (bind _sm_glass_shard_geometrycollection_sm_1_ (Variables|Default|GetSM_Glass_Shard_GeometryCollection_SM_1_))
  (bind _output_get (Variables|Default|SetDestruction%20Fragments (Utilities|Array|MakeArray _sm_glass_shard_geometrycollection_sm_1_ (Variables|Default|GetSM_Glass_Shard_GeometryCollection_SM_2_) (Variables|Default|GetSM_Glass_Shard_GeometryCollection_SM_3_) (Variables|Default|GetSM_Glass_Shard_GeometryCollection_SM_4_) (Variables|Default|GetSM_Glass_Shard_GeometryCollection_SM_5_) (Variables|Default|GetSM_Glass_Shard_GeometryCollection_SM_6_) (Variables|Default|GetSM_Glass_Shard_GeometryCollection_SM_7_) (Variables|Default|GetSM_Glass_Shard_GeometryCollection_SM_8_) (Variables|Default|GetSM_Glass_Shard_GeometryCollection_SM_9_) (Variables|Default|GetSM_Glass_Shard_GeometryCollection_SM_10_) (Variables|Default|GetSM_Glass_Shard_GeometryCollection_SM_11_) (Variables|Default|GetSM_Glass_Shard_GeometryCollection_SM_12_) (Variables|Default|GetSM_Glass_Shard_GeometryCollection_SM_13_) (Variables|Default|GetSM_Glass_Shard_GeometryCollection_SM_14_) (Variables|Default|GetSM_Glass_Shard_GeometryCollection_SM_15_) (Variables|Default|GetSM_Glass_Shard_GeometryCollection_SM_16_) (Variables|Default|GetSM_Glass_Shard_GeometryCollection_SM_17_))))
  (for _array_element _output_get
    (Rendering|Material|SetVectorParameterValueonMaterials _array_element "Pivot" (Transformation|GetWorldLocation _sm_glass_shard_geometrycollection_sm_1_))
    (Utilities|FlowControl|Delay 0.2)
    (bind _asbp_player_1 (Utilities|Casting|CastToBP_Player1 (Game|GetPlayerCharacter 0)))
    (Variables|Default|SetAs%20BP%20Player%201 _asbp_player_1)
    (bind _asbp_player_2 (Utilities|Casting|CastToBP_Player2 (Game|GetPlayerCharacter 1)))
    (Variables|Default|SetAs%20BP%20Player%202 _asbp_player_2)
    (bind _outactors (Actor|GetAllActorsOfClass "/Game/GameBehaviour/Core/Checkpoints/BP_PlayerSpawning.BP_PlayerSpawning_C"))
    (Variables|Default|SetPlayerSpawning (Utilities|Array|Get(acopy) _outactors))
    (Variables|Default|SetIsDestroyed false)
    (Collision|SetCollisionEnabled (Variables|Default|GetCollision) "QueryAndPhysics")
    (Collision|SetCollisionEnabled (Variables|Default|GetHightlightRadius) "NoCollision")
    (for _array_element_2 (Variables|Default|GetDestruction%20Fragments)
      (Rendering|SetCustomDepthStencilValue _array_element_2 (Variables|Default|GetDestroyHiglight)))))

(event EventObjectHighlight
  (params (CanBeInteractedWith :type Boolean))
  (if CanBeInteractedWith
    (if (Variables|Default|GetIsSelectedLocal)
      (for _array_element (Variables|Default|GetDestruction%20Fragments)
        (Rendering|SetRenderCustomDepth _array_element true)))))

(event EventSelectObject
  (Variables|Default|SetIsSelectedLocal true)
  (if (Variables|Default|GetIsDestroyed)
    (Utilities|IsValid (Variables|Default|GetAs%20BP%20Player%201)
      (:Is%20Valid
        (Variables|/Game/GameBehaviour/Characters/Player/SplitScreen/BP_Player1.BP_Player1_C|SetCanBeRepaired (Variables|Default|GetAs%20BP%20Player%201) true))
      (:Is%20Not%20Valid
        _))
    (Utilities|IsValid (Variables|Default|GetAs%20BP%20Player%202)
      (:Is%20Valid
        (Variables|/Game/GameBehaviour/Characters/Player/SplitScreen/BP_Player2.BP_Player2_C|SetCanBeDestroyed (Variables|Default|GetAs%20BP%20Player%202) false)))
    (else
      (Utilities|IsValid (Variables|Default|GetAs%20BP%20Player%201)
        (:Is%20Valid
          (Variables|/Game/GameBehaviour/Characters/Player/SplitScreen/BP_Player1.BP_Player1_C|SetCanBeRepaired (Variables|Default|GetAs%20BP%20Player%201) false))
        (:Is%20Not%20Valid
          _))
      (Utilities|IsValid (Variables|Default|GetAs%20BP%20Player%202)
        (:Is%20Valid
          (Variables|/Game/GameBehaviour/Characters/Player/SplitScreen/BP_Player2.BP_Player2_C|SetCanBeDestroyed (Variables|Default|GetAs%20BP%20Player%202) true))))))

(event EventRepairObject
  (params (isRepairable :type Boolean))
  (bind _collision (Variables|Default|GetCollision))
  (if true
    (Variables|/Game/GameBehaviour/Characters/Player/SplitScreen/BP_Player1.BP_Player1_C|SetCanBeRepaired (Variables|Default|GetAs%20BP%20Player%201) false)
    (Variables|/Game/GameBehaviour/Characters/Player/SplitScreen/BP_Player2.BP_Player2_C|SetCanBeDestroyed (Variables|Default|GetAs%20BP%20Player%202) true)
    (Variables|Default|SetIsDestroyed false)
    (CallFunction|DestroyedHighlight)
    (Collision|SetCollisionEnabled (Variables|Default|GetHightlightRadius) "NoCollision")
    (bind _newtrack_0 (Timeline|Timeline_3 Reverse)
      (:Update
        (for _array_element (Variables|Default|GetDestruction%20Fragments)
          (Rendering|Material|SetScalarParameterValueonMaterials _array_element "Alpha 2" _newtrack_0)
          (if (== _newtrack_0 0.0)
            (Collision|SetCollisionEnabled _collision "QueryAndPhysics")
            (else
              (Collision|SetCollisionEnabled _collision "NoCollision"))))))))

(event EventDeselectObject
  (Variables|Default|SetIsSelectedLocal false)
  (for _array_element (Variables|Default|GetDestruction%20Fragments)
    (Rendering|SetRenderCustomDepth _array_element false)))

(event EventDestructObject
  (params (isDestructable :type Boolean))
  (bind _collision (Variables|Default|GetCollision))
  (if true
    (Variables|/Game/GameBehaviour/Characters/Player/SplitScreen/BP_Player1.BP_Player1_C|SetCanBeRepaired (Variables|Default|GetAs%20BP%20Player%201) true)
    (Variables|/Game/GameBehaviour/Characters/Player/SplitScreen/BP_Player2.BP_Player2_C|SetCanBeDestroyed (Variables|Default|GetAs%20BP%20Player%202) false)
    (Variables|Default|SetIsDestroyed true)
    (CallFunction|RepairedHighlight)
    (Collision|SetCollisionEnabled (Variables|Default|GetHightlightRadius) "QueryAndPhysics")
    (bind _newtrack_0 (Timeline|Timeline_3 Play)
      (:Update
        (for _array_element (Variables|Default|GetDestruction%20Fragments)
          (Rendering|Material|SetScalarParameterValueonMaterials _array_element "Alpha 2" _newtrack_0)
          (if (== _newtrack_0 0.0)
            (Collision|SetCollisionEnabled _collision "QueryAndPhysics")
            (else
              (Collision|SetCollisionEnabled _collision "NoCollision"))))))))

(fn ConstructionScript)

(fn RepairedHighlight
  (for _array_element (Variables|Default|GetDestruction%20Fragments)
    (Rendering|SetCustomDepthStencilValue _array_element (Variables|Default|GetRepairHiglight))))

(fn DestroyedHighlight
  (for _array_element (Variables|Default|GetDestruction%20Fragments)
    (Rendering|SetCustomDepthStencilValue _array_element (Variables|Default|GetDestroyHiglight))))

(fn IsSelected
  (return false))