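; BP_Wall3 is a destructible wall of twenty box fracture pieces that animates repair through material parameters.
; BeginPlay passes the world location of one piece to all materials as a shared Pivot.
; Each RepairObject call alternately plays or reverses a timeline, whose track is split into two clamped, sequential scalars, Alpha 1 then Alpha 2, for a two-stage material-driven effect.
; IsSelected always returns false.
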(event EventBeginPlay
  (bind _box_geometrycollection_sm_6_1 (Variables|Default|GetBox_GeometryCollection_SM_6_1))
  (Rendering|Material|SetVectorParameterValueonMaterials _box_geometrycollection_sm_6_1 "Pivot" (Transformation|GetWorldLocation _box_geometrycollection_sm_6_1)))

(event EventRepairObject
  (params (isRepairable :type Boolean))
  (Development|PrintString "Activated")
  (Utilities|FlowControl|FlipFlop
    (:A
      (bind _newtrack_0 (Timeline|Timeline Play)
        (:Update
          (Rendering|Material|SetScalarParameterValueonMaterials (Variables|Default|GetBox_GeometryCollection_SM_16_1) "Alpha 1" (Math|Float|Clamp(Float) (* _newtrack_0 2.0)))
          (Rendering|Material|SetScalarParameterValueonMaterials (Variables|Default|GetBox_GeometryCollection_SM_11_1) "Alpha 2" (Math|Float|Clamp(Float) (- (* _newtrack_0 2.0) 1.0))))))
    (:B
      (Timeline|Timeline Reverse))))

(fn ConstructionScript)

(fn IsSelected
  (return false))