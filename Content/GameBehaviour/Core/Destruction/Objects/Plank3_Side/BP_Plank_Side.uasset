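; A side-scroller plank object that starts destroyed, which Player 1 can repair and Player 2 can destroy.
; A timeline plays forward to repair and in reverse to destroy, driving a material parameter on twenty mesh fragments and toggling box collision.
; A highlight radius registers the plank with overlapping players and sets their repair/destroy permissions.
; Tick toggles custom-depth highlighting when an eligible player is near, with stencil values marking repair or destroy.
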(event OnComponentBeginOverlap(HighlightRadius)
  (params (OverlappedComponent :type Primitive%20Component%20Object%20Reference) (OtherActor :type Actor%20Object%20Reference) (OtherComp :type Primitive%20Component%20Object%20Reference) (OtherBodyIndex :type Integer) (bFromSweep :type Boolean) (SweepResult :type Hit%20Result%20Structure%20%28by%20ref%29))
  (bind _as_bp_player_1_side_scroll (Variables|Default|GetAs%20BP%20Player%201%20Side%20Scroll))
  (bind _as_bp_player_2_side_scroll (Variables|Default|GetAs%20BP%20Player%202%20Side%20Scroll))
  (Utilities|Casting|CastToBP_Player1_SideScroll OtherActor
    (:then
      (Variables|Default|SetisPlayer1Overlapping true)
      (Variables|/Game/GameBehaviour/Characters/Player/SideScroll/BP_Player1_SideScroll.BP_Player1_SideScroll_C|SetrepairingObject _as_bp_player_1_side_scroll self)
      (if (Variables|Default|GetIsDestroyed)
        (CallFunction|RepairedHighlight)
        (Variables|/Game/GameBehaviour/Characters/Player/SideScroll/BP_Player1_SideScroll.BP_Player1_SideScroll_C|SetcanRepair _as_bp_player_1_side_scroll true)
        (Variables|/Game/GameBehaviour/Characters/Player/SideScroll/BP_Player2_SideScroll.BP_Player2_SideScroll_C|SetcanDestroy (Variables|Default|GetAs%20BP%20Player%202%20Side%20Scroll) false)))
    (:CastFailed
      (Utilities|Casting|CastToBP_Player2_SideScroll OtherActor)
      (Variables|Default|SetisPlayer2Overlapping true)
      (Variables|/Game/GameBehaviour/Characters/Player/SideScroll/BP_Player2_SideScroll.BP_Player2_SideScroll_C|SetrepairingObject _as_bp_player_2_side_scroll self)
      (if (not (Variables|Default|GetIsDestroyed))
        (CallFunction|DestroyedHighlight)
        (Variables|/Game/GameBehaviour/Characters/Player/SideScroll/BP_Player1_SideScroll.BP_Player1_SideScroll_C|SetcanRepair (Variables|Default|GetAs%20BP%20Player%201%20Side%20Scroll) false)
        (Variables|/Game/GameBehaviour/Characters/Player/SideScroll/BP_Player2_SideScroll.BP_Player2_SideScroll_C|SetcanDestroy _as_bp_player_2_side_scroll true)))))

(event OnComponentEndOverlap(HighlightRadius)
  (params (OverlappedComponent :type Primitive%20Component%20Object%20Reference) (OtherActor :type Actor%20Object%20Reference) (OtherComp :type Primitive%20Component%20Object%20Reference) (OtherBodyIndex :type Integer))
  (bind _as_bp_player_2_side_scroll (Variables|Default|GetAs%20BP%20Player%202%20Side%20Scroll))
  (bind _as_bp_player_1_side_scroll (Variables|Default|GetAs%20BP%20Player%201%20Side%20Scroll))
  (Utilities|Casting|CastToBP_Player1_SideScroll OtherActor
    (:then
      (Variables|Default|SetisPlayer1Overlapping false)
      (Variables|/Game/GameBehaviour/Characters/Player/SideScroll/BP_Player1_SideScroll.BP_Player1_SideScroll_C|SetcanRepair _as_bp_player_1_side_scroll false)
      (Variables|/Game/GameBehaviour/Characters/Player/SideScroll/BP_Player1_SideScroll.BP_Player1_SideScroll_C|SetrepairingObject _as_bp_player_1_side_scroll 0))
    (:CastFailed
      (Utilities|Casting|CastToBP_Player2_SideScroll OtherActor)
      (Variables|Default|SetisPlayer2Overlapping false)
      (Variables|/Game/GameBehaviour/Characters/Player/SideScroll/BP_Player2_SideScroll.BP_Player2_SideScroll_C|SetcanDestroy _as_bp_player_2_side_scroll false)
      (Variables|/Game/GameBehaviour/Characters/Player/SideScroll/BP_Player2_SideScroll.BP_Player2_SideScroll_C|SetrepairingObject _as_bp_player_2_side_scroll 0))))

(event EventBeginPlay
  (bind _sm_plank_side_1_ (Variables|Default|GetSM_Plank_Side_1_))
  (bind _output_get (Variables|Default|SetDestruction%20Fragments (Utilities|Array|MakeArray _sm_plank_side_1_ (Variables|Default|GetSM_Plank_Side_2_) (Variables|Default|GetSM_Plank_Side_3_) (Variables|Default|GetSM_Plank_Side_4_) (Variables|Default|GetSM_Plank_Side_5_) (Variables|Default|GetSM_Plank_Side_6_) (Variables|Default|GetSM_Plank_Side_7_) (Variables|Default|GetSM_Plank_Side_8_) (Variables|Default|GetSM_Plank_Side_9_) (Variables|Default|GetSM_Plank_Side_10_) (Variables|Default|GetSM_Plank_Side_11_) (Variables|Default|GetSM_Plank_Side_12_) (Variables|Default|GetSM_Plank_Side_13_) (Variables|Default|GetSM_Plank_Side_14_) (Variables|Default|GetSM_Plank_Side_15_) (Variables|Default|GetSM_Plank_Side_16_) (Variables|Default|GetSM_Plank_Side_17_) (Variables|Default|GetSM_Plank_Side_18_) (Variables|Default|GetSM_Plank_Side_19_) (Variables|Default|GetSM_Plank_Side_20_))))
  (for _array_element _output_get
    (Rendering|Material|SetVectorParameterValueonMaterials _array_element "Pivot" (Transformation|GetWorldLocation _sm_plank_side_1_))
    (Utilities|FlowControl|Delay 0.2)
    (bind _asbp_player_1_side_scroll (Utilities|Casting|CastToBP_Player1_SideScroll (Game|GetPlayerCharacter 0)))
    (Variables|Default|SetAs%20BP%20Player%201%20Side%20Scroll _asbp_player_1_side_scroll)
    (bind _asbp_player_2_side_scroll (Utilities|Casting|CastToBP_Player2_SideScroll (Game|GetPlayerCharacter 1)))
    (Variables|Default|SetAs%20BP%20Player%202%20Side%20Scroll _asbp_player_2_side_scroll)
    (Variables|Default|SetIsDestroyed true)
    (for _array_element_2 (Variables|Default|GetDestruction%20Fragments)
      (Collision|SetCollisionEnabled _array_element_2 "NoCollision")
      (Rendering|SetCustomDepthStencilValue _array_element_2 (Variables|Default|GetRepairHiglight)))))

(event EventObjectHighlight
  (params (CanBeInteractedWith :type Boolean))
  (if CanBeInteractedWith
    (for _array_element (Variables|Default|GetDestruction%20Fragments)
      (Rendering|SetRenderCustomDepth _array_element true))))

(event EventSelectObject)

(event EventRepairObject
  (params (isRepairable :type Boolean))
  (if true
    (Variables|/Game/GameBehaviour/Characters/Player/SideScroll/BP_Player1_SideScroll.BP_Player1_SideScroll_C|SetcanRepair (Variables|Default|GetAs%20BP%20Player%201%20Side%20Scroll) false)
    (Variables|/Game/GameBehaviour/Characters/Player/SideScroll/BP_Player2_SideScroll.BP_Player2_SideScroll_C|SetcanDestroy (Variables|Default|GetAs%20BP%20Player%202%20Side%20Scroll) true)
    (Variables|Default|SetIsDestroyed false)
    (CallFunction|DestroyedHighlight)
    (bind _newtrack_0 (Timeline|Timeline Play)
      (:Update
        (for _array_element (Variables|Default|GetDestruction%20Fragments)
          (Rendering|Material|SetScalarParameterValueonMaterials _array_element "Alpha 2" _newtrack_0)
          (if (== _newtrack_0 0.0)
            (Collision|SetCollisionEnabled (Variables|Default|GetBox) "QueryAndPhysics")
            (else
              (Collision|SetCollisionEnabled (Variables|Default|GetBox) "NoCollision"))))))))

(event EventDeselectObject
  (Variables|Default|SetIsSelectedLocal false)
  (for _array_element (Variables|Default|GetDestruction%20Fragments)
    (Rendering|SetRenderCustomDepth _array_element false)))

(event EventDestructObject
  (params (isDestructable :type Boolean))
  (if true
    (Variables|/Game/GameBehaviour/Characters/Player/SideScroll/BP_Player1_SideScroll.BP_Player1_SideScroll_C|SetcanRepair (Variables|Default|GetAs%20BP%20Player%201%20Side%20Scroll) true)
    (Variables|/Game/GameBehaviour/Characters/Player/SideScroll/BP_Player2_SideScroll.BP_Player2_SideScroll_C|SetcanDestroy (Variables|Default|GetAs%20BP%20Player%202%20Side%20Scroll) false)
    (Variables|Default|SetIsDestroyed true)
    (CallFunction|RepairedHighlight)
    (bind _newtrack_0 (Timeline|Timeline Reverse)
      (:Update
        (for _array_element (Variables|Default|GetDestruction%20Fragments)
          (Rendering|Material|SetScalarParameterValueonMaterials _array_element "Alpha 2" _newtrack_0)
          (if (== _newtrack_0 0.0)
            (Collision|SetCollisionEnabled (Variables|Default|GetBox) "QueryAndPhysics")
            (else
              (Collision|SetCollisionEnabled (Variables|Default|GetBox) "NoCollision"))))))))

(event EventTick
  (params (DeltaSeconds :type Float%20%28single-precision%29))
  (if (Variables|Default|GetisPlayer1Overlapping)
    (if (Variables|Default|GetIsDestroyed)
      (CallFunction|ObjectHighlight true :!label _label)
      (elif (Variables|Default|GetisPlayer2Overlapping)
        (goto _label)
        (else
          (CallFunction|DeselectObject))))
    (elif (Variables|Default|GetisPlayer2Overlapping)
      (if (Variables|Default|GetIsDestroyed)
        (if (Variables|Default|GetisPlayer1Overlapping)
          (CallFunction|ObjectHighlight true :!label _label_2)
          (else
            (CallFunction|DeselectObject)))
        (else
          (goto _label_2)))
      (else
        (CallFunction|DeselectObject)))))

(fn ConstructionScript)

(fn RepairedHighlight
  (for _array_element (Variables|Default|GetDestruction%20Fragments)
    (Rendering|SetCustomDepthStencilValue _array_element (Variables|Default|GetRepairHiglight))))

(fn DestroyedHighlight
  (for _array_element (Variables|Default|GetDestruction%20Fragments)
    (Rendering|SetCustomDepthStencilValue _array_element (Variables|Default|GetDestroyHiglight))))

(fn IsSelected
  (return false))