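; Football minigame actor that tracks goals scored in two goals with a physics ball.
; Each goal's overlap with the ball increments that side's score, capped at 99, and updates its text display.
; Scoring, or the ball leaving the BallRange volume, calls RespawnBall, which moves it to the respawn point and zeroes its linear and angular velocity.
; The ball is also placed at the respawn point on BeginPlay.
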(event OnComponentBeginOverlap(Goal1)
  (params (OverlappedComponent :type Primitive%20Component%20Object%20Reference) (OtherActor :type Actor%20Object%20Reference) (OtherComp :type Primitive%20Component%20Object%20Reference) (OtherBodyIndex :type Integer) (bFromSweep :type Boolean) (SweepResult :type Hit%20Result%20Structure%20%28by%20ref%29))
  (if (== OtherComp (Variables|Default|GetFootball))
    (CallFunction|RespawnBall)
    (if (< (Variables|Default|GetScore1) 99)
      (bind _output_get (Variables|Default|SetScore1 (+ (Variables|Default|GetScore1) 1)))
      (Rendering|Components|TextRender|SetText (Variables|Default|GetGoal1Score) (Utilities|Text|ToText(Integer) _output_get)))))

(event OnComponentBeginOverlap(Goal2)
  (params (OverlappedComponent :type Primitive%20Component%20Object%20Reference) (OtherActor :type Actor%20Object%20Reference) (OtherComp :type Primitive%20Component%20Object%20Reference) (OtherBodyIndex :type Integer) (bFromSweep :type Boolean) (SweepResult :type Hit%20Result%20Structure%20%28by%20ref%29))
  (if (== OtherComp (Variables|Default|GetFootball))
    (CallFunction|RespawnBall)
    (if (< (Variables|Default|GetScore2) 99)
      (bind _output_get (Variables|Default|SetScore2 (+ (Variables|Default|GetScore2) 1)))
      (Rendering|Components|TextRender|SetText (Variables|Default|GetGoal2Score) (Utilities|Text|ToText(Integer) _output_get)))))

(event OnComponentEndOverlap(BallRange)
  (params (OverlappedComponent :type Primitive%20Component%20Object%20Reference) (OtherActor :type Actor%20Object%20Reference) (OtherComp :type Primitive%20Component%20Object%20Reference) (OtherBodyIndex :type Integer))
  (if (== OtherComp (Variables|Default|GetFootball))
    (CallFunction|RespawnBall)))

(event EventBeginPlay
  (Transformation|SetWorldLocation (Variables|Default|GetFootball) (Transformation|GetWorldLocation (Variables|Default|GetBallRespawnLocation)) false false))

(fn ConstructionScript)

(fn RespawnBall
  (Transformation|SetWorldLocation (Variables|Default|GetFootball) (Transformation|GetWorldLocation (Variables|Default|GetBallRespawnLocation)) false false)
  (Physics|SetPhysicsLinearVelocity (Variables|Default|GetFootball) "0, 0, 0" false "None")
  (Class|PrimitiveComponent|SetPhysicsAngularVelocityinDegrees (Variables|Default|GetFootball) "0, 0, 0" false "None"))