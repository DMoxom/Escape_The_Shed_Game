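; Pushable block for two players that can only be moved physically while a player is touching one of its trigger boxes.
; XBox and YBox overlap events check the Player1 and Player2 actor tags to set a per-player overlap flag.
; Tick enables physics simulation on the Object component while either flag is set, and uses a re-armed DoOnce to switch it off once both clear.
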(event OnComponentBeginOverlap(yBox)
  (params (OverlappedComponent :type Primitive%20Component%20Object%20Reference) (OtherActor :type Actor%20Object%20Reference) (OtherComp :type Primitive%20Component%20Object%20Reference) (OtherBodyIndex :type Integer) (bFromSweep :type Boolean) (SweepResult :type Hit%20Result%20Structure%20%28by%20ref%29))
  (if (Actor|ActorHasTag OtherActor "Player1")
    (Variables|Default|SetPlayer1Overlapping true)
    (elif (Actor|ActorHasTag OtherActor "Player2")
      (Variables|Default|SetPlayer2Overlapping true))))

(event OnComponentEndOverlap(yBox)
  (params (OverlappedComponent :type Primitive%20Component%20Object%20Reference) (OtherActor :type Actor%20Object%20Reference) (OtherComp :type Primitive%20Component%20Object%20Reference) (OtherBodyIndex :type Integer))
  (if (Actor|ActorHasTag OtherActor "Player1")
    (Variables|Default|SetPlayer1Overlapping false)
    (elif (Actor|ActorHasTag OtherActor "Player2")
      (Variables|Default|SetPlayer2Overlapping false))))

(event OnComponentBeginOverlap(xBox)
  (params (OverlappedComponent :type Primitive%20Component%20Object%20Reference) (OtherActor :type Actor%20Object%20Reference) (OtherComp :type Primitive%20Component%20Object%20Reference) (OtherBodyIndex :type Integer) (bFromSweep :type Boolean) (SweepResult :type Hit%20Result%20Structure%20%28by%20ref%29))
  (if (Actor|ActorHasTag OtherActor "Player1")
    (Variables|Default|SetPlayer1Overlapping true)
    (elif (Actor|ActorHasTag OtherActor "Player2")
      (Variables|Default|SetPlayer2Overlapping true))))

(event OnComponentEndOverlap(xBox)
  (params (OverlappedComponent :type Primitive%20Component%20Object%20Reference) (OtherActor :type Actor%20Object%20Reference) (OtherComp :type Primitive%20Component%20Object%20Reference) (OtherBodyIndex :type Integer))
  (if (Actor|ActorHasTag OtherActor "Player1")
    (Variables|Default|SetPlayer1Overlapping false)
    (elif (Actor|ActorHasTag OtherActor "Player2")
      (Variables|Default|SetPlayer2Overlapping false))))

(event EventBeginPlay)

(event Collision|EventActorBeginOverlap
  (params (OtherActor :type Actor%20Object%20Reference)))

(event EventTick
  (params (DeltaSeconds :type Float%20%28single-precision%29))
  (if (or (Variables|Default|GetPlayer1Overlapping) (Variables|Default|GetPlayer2Overlapping))
    (Physics|SetSimulatePhysics (Variables|Default|GetObject) true)
    (goto _label Reset)
    (else
      (Utilities|FlowControl|DoOnce false :!label _label
        (:Completed
          (Physics|SetSimulatePhysics (Variables|Default|GetObject) false))))))

(fn ConstructionScript)