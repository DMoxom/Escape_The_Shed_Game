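; BP_CollectiblePotShard is a pot shard collectible that the player picks up by touching it.
; When an actor tagged Player1 overlaps its Box, it decrements PotShardsLeft on the OptionsGameInstance and sends the new count to the CollectibleController and its widget to update the pot message.
; It then writes its Index slot in the game instance's Collectibles array and destroys itself.
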(event OnComponentBeginOverlap(Box)
  (params (OverlappedComponent :type Primitive%20Component%20Object%20Reference) (OtherActor :type Actor%20Object%20Reference) (OtherComp :type Primitive%20Component%20Object%20Reference) (OtherBodyIndex :type Integer) (bFromSweep :type Boolean) (SweepResult :type Hit%20Result%20Structure%20%28by%20ref%29))
  (bind _collectiblecontroller (Variables|Default|GetCollectibleController))
  (bind _optionsgameinstance (Variables|Default|GetOptionsGameInstance))
  (if (Actor|ActorHasTag OtherActor "Player1")
    (bind _result (Math|Integer|DecrementInt (Variables|/Game/GameBehaviour/Core/GameInstance/OptionsGameInstance.OptionsGameInstance_C|GetPotShardsLeft _optionsgameinstance))
      (:%20%20
        (bind _output_get (Variables|/Game/GameBehaviour/Core/GameInstance/OptionsGameInstance.OptionsGameInstance_C|SetPotShardsLeft _optionsgameinstance _result))
        (Class|BICollectibleSystem|UpdatePot(Message) (Variables|/Game/GameBehaviour/Core/Collectibles/Collectables/BP_CollectibleController.BP_CollectibleController_C|GetCollectibleWidget _collectiblecontroller) _output_get)
        (Class|BICollectibleSystem|UpdatePot(Message) _collectiblecontroller _output_get)
        (Utilities|Array|SetArrayElem (Variables|/Game/GameBehaviour/Core/GameInstance/OptionsGameInstance.OptionsGameInstance_C|GetCollectibles (Variables|Default|GetOptionsGameInstance)) (Variables|Default|GetIndex) false)
        (Actor|DestroyActor)))))

(event EventBeginPlay
  (|CallParentFunction))

(fn ConstructionScript
  (|CallParentFunction))