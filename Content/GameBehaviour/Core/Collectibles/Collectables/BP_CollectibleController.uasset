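; Level controller for key, pot shard and fluff collectibles that tracks totals, unlocks rewards and applies both players' chosen hats.
; On BeginPlay it counts and indexes collectibles, removes pot shards and fluff already flagged collected in OptionsGameInstance, and creates the counter widget.
; Collecting every key enables the side-scroll map activator.
; Completing pot shards or fluff unlocks a Player 1 or Player 2 hat respectively, based on current level.
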(event EventBeginPlay
  (bind _asoptions_game_instance (Utilities|Casting|CastToOptionsGameInstance (Game|GetGameInstance)))
  (Variables|Default|SetOptionsGameInstance _asoptions_game_instance)
  (Utilities|FlowControl|Sequence
    (:then_0
      (Utilities|FlowControl|Delay 0.2)
      (bind _returnvalue (Actor|GetActorOfClass "/Game/GameBehaviour/Characters/Player/SplitScreen/BP_Player1.BP_Player1_C"))
      (Variables|Default|SetPlayer1 _returnvalue)
      (bind _returnvalue_2 (Actor|GetActorOfClass "/Game/GameBehaviour/Characters/Player/SideScroll/BP_Player1_SideScroll.BP_Player1_SideScroll_C"))
      (Variables|Default|SetPlayer1SideScroll _returnvalue_2)
      (bind _returnvalue_3 (Actor|GetActorOfClass "/Game/GameBehaviour/Characters/Player/SplitScreen/BP_Player2.BP_Player2_C"))
      (Variables|Default|SetPlayer2 _returnvalue_3)
      (bind _returnvalue_4 (Actor|GetActorOfClass "/Game/GameBehaviour/Characters/Player/SideScroll/BP_Player2_SideScroll.BP_Player2_SideScroll_C"))
      (Variables|Default|SetPlayer2SideScroll _returnvalue_4)
      (CallFunction|ToggleHats))
    (:then_1
      (bind _outactors (Actor|GetAllActorsOfClass "/Game/GameBehaviour/Core/Collectibles/Collectables/BP_CollectibleKey.BP_CollectibleKey_C"))
      (Variables|/Game/GameBehaviour/Core/GameInstance/OptionsGameInstance.OptionsGameInstance_C|SetKeysTotal (Variables|Default|GetOptionsGameInstance) (Utilities|Array|Length _outactors))
      (bind _outactors_2 (Actor|GetAllActorsOfClass "/Game/GameBehaviour/Core/Collectibles/Collectables/BP_CollectiblePotShard.BP_CollectiblePotShard_C"))
      (Variables|/Game/GameBehaviour/Core/GameInstance/OptionsGameInstance.OptionsGameInstance_C|SetPotShardsTotal (Variables|Default|GetOptionsGameInstance) (Utilities|Array|Length _outactors_2))
      (bind _outactors_3 (Actor|GetAllActorsOfClass "/Game/GameBehaviour/Core/Collectibles/Collectables/BP_CollectibleFluff.BP_CollectibleFluff_C"))
      (Variables|/Game/GameBehaviour/Core/GameInstance/OptionsGameInstance.OptionsGameInstance_C|SetFluffTotal (Variables|Default|GetOptionsGameInstance) (Utilities|Array|Length _outactors_3))
      (Variables|/Game/GameBehaviour/Core/GameInstance/OptionsGameInstance.OptionsGameInstance_C|SetKeysLeft (Variables|Default|GetOptionsGameInstance) (Variables|/Game/GameBehaviour/Core/GameInstance/OptionsGameInstance.OptionsGameInstance_C|GetKeysTotal (Variables|Default|GetOptionsGameInstance)))
      (Variables|/Game/GameBehaviour/Core/GameInstance/OptionsGameInstance.OptionsGameInstance_C|SetFluffLeft (Variables|Default|GetOptionsGameInstance) (Variables|/Game/GameBehaviour/Core/GameInstance/OptionsGameInstance.OptionsGameInstance_C|GetFluffTotal (Variables|Default|GetOptionsGameInstance)))
      (Variables|/Game/GameBehaviour/Core/GameInstance/OptionsGameInstance.OptionsGameInstance_C|SetPotShardsLeft (Variables|Default|GetOptionsGameInstance) (Variables|/Game/GameBehaviour/Core/GameInstance/OptionsGameInstance.OptionsGameInstance_C|GetPotShardsTotal (Variables|Default|GetOptionsGameInstance))))
    (:then_2
      (bind _outactors_4 (Actor|GetAllActorsOfClass "/Game/GameBehaviour/Core/Collectibles/Collectables/BP_BaseCollectible.BP_BaseCollectible_C"))
      (Variables|Default|SetCollectibles _outactors_4)
      (for (_array_element _array_index) _outactors_4
        (Variables|/Game/GameBehaviour/Core/Collectibles/Collectables/BP_BaseCollectible.BP_BaseCollectible_C|SetIndex _array_element _array_index))
      (if (Utilities|Array|IsEmpty (Variables|/Game/GameBehaviour/Core/GameInstance/OptionsGameInstance.OptionsGameInstance_C|GetCollectibles (Variables|Default|GetOptionsGameInstance)))
        (for _array_element_2 (Variables|Default|GetCollectibles)
          (Utilities|Array|Add (Variables|/Game/GameBehaviour/Core/GameInstance/OptionsGameInstance.OptionsGameInstance_C|GetCollectibles (Variables|Default|GetOptionsGameInstance)) true))
        (else
          (for (_array_element_3 _array_index_2) (Variables|Default|GetCollectibles)
            (Variables|Default|SetCollectible _array_element_3)
            (if (not (Utilities|Array|Get(acopy) (Variables|/Game/GameBehaviour/Core/GameInstance/OptionsGameInstance.OptionsGameInstance_C|GetCollectibles (Variables|Default|GetOptionsGameInstance)) _array_index_2))
              (if (Actor|ActorHasTag (Variables|Default|GetCollectible) "Fluff")
                (Variables|/Game/GameBehaviour/Core/GameInstance/OptionsGameInstance.OptionsGameInstance_C|SetFluffLeft (Variables|Default|GetOptionsGameInstance) (- (Variables|/Game/GameBehaviour/Core/GameInstance/OptionsGameInstance.OptionsGameInstance_C|GetFluffLeft (Variables|Default|GetOptionsGameInstance)) 1))
                (Actor|DestroyActor (Variables|Default|GetCollectible))
                (elif (Actor|ActorHasTag (Variables|Default|GetCollectible) "PotShard")
                  (Variables|/Game/GameBehaviour/Core/GameInstance/OptionsGameInstance.OptionsGameInstance_C|SetPotShardsLeft (Variables|Default|GetOptionsGameInstance) (- (Variables|/Game/GameBehaviour/Core/GameInstance/OptionsGameInstance.OptionsGameInstance_C|GetPotShardsLeft (Variables|Default|GetOptionsGameInstance)) 1))
                  (Actor|DestroyActor (Variables|Default|GetCollectible)))))))))
    (:then_3
      (bind _returnvalue_5 (UserInterface|CreateWidget "/Game/GameBehaviour/UI/Widgets/WBP_Collectibles.WBP_Collectibles_C"))
      (bind _output_get (Variables|Default|SetCollectibleWidget _returnvalue_5))
      (UserInterface|Viewport|AddtoViewport _output_get 0)
      (Class|BICollectibleSystem|WidgetSetup(Message) (Variables|Default|GetCollectibleWidget) (Variables|/Game/GameBehaviour/Core/GameInstance/OptionsGameInstance.OptionsGameInstance_C|GetKeysTotal (Variables|Default|GetOptionsGameInstance)) (Variables|/Game/GameBehaviour/Core/GameInstance/OptionsGameInstance.OptionsGameInstance_C|GetPotShardsTotal (Variables|Default|GetOptionsGameInstance)) (Variables|/Game/GameBehaviour/Core/GameInstance/OptionsGameInstance.OptionsGameInstance_C|GetFluffTotal (Variables|Default|GetOptionsGameInstance)))
      (Default|UpdatePot (Variables|Default|GetCollectibleWidget) (Variables|/Game/GameBehaviour/Core/GameInstance/OptionsGameInstance.OptionsGameInstance_C|GetPotShardsLeft (Variables|Default|GetOptionsGameInstance)))
      (Default|UpdateFluff (Variables|Default|GetCollectibleWidget) (Variables|/Game/GameBehaviour/Core/GameInstance/OptionsGameInstance.OptionsGameInstance_C|GetFluffLeft (Variables|Default|GetOptionsGameInstance))))
    (:then_4
      (bind _outactors_5 (Actor|GetAllActorsOfClass "/Game/GameBehaviour/Core/NewButtonSystem/BP_ActivatorBase_Load_SideScrollMap.BP_ActivatorBase_Load_SideScrollMap_C"))
      (Variables|Default|SetActivatorSideScroll (Utilities|Array|Get(acopy) _outactors_5)))))

(event EventUpdatePot
  (params (PotLeft :type Integer))
  (bind _optionsgameinstance (Variables|Default|GetOptionsGameInstance))
  (bind _optionsgameinstance_2 (Variables|Default|GetOptionsGameInstance))
  (if (== PotLeft 0)
    (if (== (Variables|/Game/GameBehaviour/Core/GameInstance/OptionsGameInstance.OptionsGameInstance_C|GetCurrentLevel (Variables|Default|GetOptionsGameInstance)) 0)
      (if (< (Variables|/Game/GameBehaviour/Core/GameInstance/OptionsGameInstance.OptionsGameInstance_C|GetPlayer1HatNumUnlocked _optionsgameinstance) 1)
        (Variables|/Game/GameBehaviour/Core/GameInstance/OptionsGameInstance.OptionsGameInstance_C|SetPlayer1HatNumUnlocked _optionsgameinstance 1))
      (elif (< (Variables|/Game/GameBehaviour/Core/GameInstance/OptionsGameInstance.OptionsGameInstance_C|GetPlayer1HatNumUnlocked _optionsgameinstance_2) 2)
        (Variables|/Game/GameBehaviour/Core/GameInstance/OptionsGameInstance.OptionsGameInstance_C|SetPlayer1HatNumUnlocked _optionsgameinstance_2 2)))))

(event EventUpdateKey
  (params (KeyLeft :type Integer))
  (if (== KeyLeft 0)
    (Class|BIButtonQuick|CanUseButton(Message) (Variables|Default|GetActivatorSideScroll) true)))

(event EventUpdateFluff
  (params (FluffLeft :type Integer))
  (bind _optionsgameinstance (Variables|Default|GetOptionsGameInstance))
  (bind _optionsgameinstance_2 (Variables|Default|GetOptionsGameInstance))
  (if (== FluffLeft 0)
    (if (== (Variables|/Game/GameBehaviour/Core/GameInstance/OptionsGameInstance.OptionsGameInstance_C|GetCurrentLevel (Variables|Default|GetOptionsGameInstance)) 0)
      (if (< (Variables|/Game/GameBehaviour/Core/GameInstance/OptionsGameInstance.OptionsGameInstance_C|GetPlayer2HatNumUnlocked _optionsgameinstance_2) 1)
        (Variables|/Game/GameBehaviour/Core/GameInstance/OptionsGameInstance.OptionsGameInstance_C|SetPlayer2HatNumUnlocked _optionsgameinstance_2 1))
      (elif (< (Variables|/Game/GameBehaviour/Core/GameInstance/OptionsGameInstance.OptionsGameInstance_C|GetPlayer2HatNumUnlocked _optionsgameinstance) 2)
        (Variables|/Game/GameBehaviour/Core/GameInstance/OptionsGameInstance.OptionsGameInstance_C|SetPlayer2HatNumUnlocked _optionsgameinstance 2)))))

(fn ConstructionScript)

(fn ToggleHats
  (bind _returnvalue (Game|GetCurrentLevelName true))
  (if (Utilities|Enum|Equal(Enum) _returnvalue "SideScrollTestMap")
    (Rendering|SetVisibility (Variables|/Game/GameBehaviour/Characters/Player/SideScroll/BP_Player1_SideScroll.BP_Player1_SideScroll_C|GetBoo_Hat (Variables|Default|GetPlayer1SideScroll)) false false)
    (Rendering|SetVisibility (Variables|/Game/GameBehaviour/Characters/Player/SideScroll/BP_Player1_SideScroll.BP_Player1_SideScroll_C|GetSM_Tophat (Variables|Default|GetPlayer1SideScroll)) false false)
    (Rendering|SetVisibility (Variables|/Game/GameBehaviour/Characters/Player/SideScroll/BP_Player2_SideScroll.BP_Player2_SideScroll_C|GetBoo_Hat (Variables|Default|GetPlayer2SideScroll)) false false)
    (Rendering|SetVisibility (Variables|/Game/GameBehaviour/Characters/Player/SideScroll/BP_Player2_SideScroll.BP_Player2_SideScroll_C|GetSM_Tophat (Variables|Default|GetPlayer2SideScroll)) false false)
    (if (== (Variables|/Game/GameBehaviour/Core/GameInstance/OptionsGameInstance.OptionsGameInstance_C|GetPlayer1HatNum (Variables|Default|GetOptionsGameInstance)) 1)
      (Rendering|ToggleVisibility (Variables|/Game/GameBehaviour/Characters/Player/SideScroll/BP_Player1_SideScroll.BP_Player1_SideScroll_C|GetBoo_Hat (Variables|Default|GetPlayer1SideScroll)) true))
    (if (== (Variables|/Game/GameBehaviour/Core/GameInstance/OptionsGameInstance.OptionsGameInstance_C|GetPlayer1HatNum (Variables|Default|GetOptionsGameInstance)) 2)
      (Rendering|ToggleVisibility (Variables|/Game/GameBehaviour/Characters/Player/SideScroll/BP_Player1_SideScroll.BP_Player1_SideScroll_C|GetSM_Tophat (Variables|Default|GetPlayer1SideScroll)) true))
    (if (== (Variables|/Game/GameBehaviour/Core/GameInstance/OptionsGameInstance.OptionsGameInstance_C|GetPlayer2HatNum (Variables|Default|GetOptionsGameInstance)) 1)
      (Rendering|ToggleVisibility (Variables|/Game/GameBehaviour/Characters/Player/SideScroll/BP_Player2_SideScroll.BP_Player2_SideScroll_C|GetBoo_Hat (Variables|Default|GetPlayer2SideScroll)) true))
    (if (== (Variables|/Game/GameBehaviour/Core/GameInstance/OptionsGameInstance.OptionsGameInstance_C|GetPlayer2HatNum (Variables|Default|GetOptionsGameInstance)) 2)
      (Rendering|ToggleVisibility (Variables|/Game/GameBehaviour/Characters/Player/SideScroll/BP_Player2_SideScroll.BP_Player2_SideScroll_C|GetSM_Tophat (Variables|Default|GetPlayer2SideScroll)) true))
    (else
      (Rendering|SetVisibility (Variables|/Game/GameBehaviour/Characters/Player/SplitScreen/BP_Player1.BP_Player1_C|GetBoo_Hat (Variables|Default|GetPlayer1)) false false)
      (Rendering|SetVisibility (Variables|/Game/GameBehaviour/Characters/Player/SplitScreen/BP_Player1.BP_Player1_C|GetSM_Tophat (Variables|Default|GetPlayer1)) false false)
      (Rendering|SetVisibility (Variables|/Game/GameBehaviour/Characters/Player/SplitScreen/BP_Player2.BP_Player2_C|GetBoo_Hat (Variables|Default|GetPlayer2)) false false)
      (Rendering|SetVisibility (Variables|/Game/GameBehaviour/Characters/Player/SplitScreen/BP_Player2.BP_Player2_C|GetSM_Tophat (Variables|Default|GetPlayer2)) false false)
      (if (== (Variables|/Game/GameBehaviour/Core/GameInstance/OptionsGameInstance.OptionsGameInstance_C|GetPlayer1HatNum (Variables|Default|GetOptionsGameInstance)) 1)
        (Rendering|ToggleVisibility (Variables|/Game/GameBehaviour/Characters/Player/SplitScreen/BP_Player1.BP_Player1_C|GetBoo_Hat (Variables|Default|GetPlayer1)) true))
      (if (== (Variables|/Game/GameBehaviour/Core/GameInstance/OptionsGameInstance.OptionsGameInstance_C|GetPlayer1HatNum (Variables|Default|GetOptionsGameInstance)) 2)
        (Rendering|ToggleVisibility (Variables|/Game/GameBehaviour/Characters/Player/SplitScreen/BP_Player1.BP_Player1_C|GetSM_Tophat (Variables|Default|GetPlayer1)) true))
      (if (== (Variables|/Game/GameBehaviour/Core/GameInstance/OptionsGameInstance.OptionsGameInstance_C|GetPlayer2HatNum (Variables|Default|GetOptionsGameInstance)) 1)
        (Rendering|ToggleVisibility (Variables|/Game/GameBehaviour/Characters/Player/SplitScreen/BP_Player2.BP_Player2_C|GetBoo_Hat (Variables|Default|GetPlayer2)) true))
      (if (== (Variables|/Game/GameBehaviour/Core/GameInstance/OptionsGameInstance.OptionsGameInstance_C|GetPlayer2HatNum (Variables|Default|GetOptionsGameInstance)) 2)
        (Rendering|ToggleVisibility (Variables|/Game/GameBehaviour/Characters/Player/SplitScreen/BP_Player2.BP_Player2_C|GetSM_Tophat (Variables|Default|GetPlayer2)) true)))))