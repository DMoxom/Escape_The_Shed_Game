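; Test game mode that sets up two-player local co-op with BP_Player1 and BP_Player2.
; On BeginPlay it removes the existing players, creates both by switching DefaultPawnClass, and teleports player one to a fixed location.
; Destroy events on both initial pawns trigger a delayed respawn and possession, but replacement pawns are never rebound and Respawn is empty.
; Unconnected nodes hold abandoned controller-assignment attempts, and SpawnPlayer2 has no caller here.
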(event Custom|OnDestroyed_
  (params (DestroyedActor :type Actor%20Object%20Reference))
  ;[1 1 1] Checks to see which player was destroyed and respawns them accordingly
  (if (== DestroyedActor (stale EventBeginPlay _asbp_player_1))
    (Utilities|FlowControl|Delay 0.5)
    (bind _returnvalue (Game|SpawnActorfromClass "/Game/GameBehaviour/Characters/Player/BP_Player1.BP_Player1_C" (Variables|Default|GetSpawnLocation) "Undefined" 0 0))
    (Pawn|Possess (Game|GetPlayerController 0) _returnvalue)
    (CallFunction|Respawn)
    (else
      (Utilities|FlowControl|Delay 0.5)
      (bind _returnvalue_2 (Game|SpawnActorfromClass "/Game/GameBehaviour/Characters/Player/BP_Player2.BP_Player2_C" (Variables|Default|GetSpawnLocation2) "Undefined" 0 0))
      (Pawn|Possess (Game|GetPlayerController 1) _returnvalue_2)
      (CallFunction|Respawn))))

(event Custom|SpawnPlayers
  ;[1 1 1] This will spawn the default third person player, delete it and then spawn player 1 and player 2
  (Class|GameplayStatics|RemovePlayer (Game|GetPlayerController 0) true)
  (Class|GameplayStatics|RemovePlayer (Game|GetPlayerController 1) true)
  (Variables|Default|SetDefaultPawnClass "/Game/GameBehaviour/Characters/Player/BP_Player1.BP_Player1_C")
  (Class|GameplayStatics|CreatePlayer 0)
  (Variables|Default|SetDefaultPawnClass "/Game/GameBehaviour/Characters/Player/BP_Player2.BP_Player2_C")
  (Class|GameplayStatics|CreatePlayer 1)
  (Transformation|SetActorLocation (Game|GetPlayerCharacter 0) "800.000000,5565.000000,542.000000" false false))

(event Custom|SpawnPlayer2
  ;[0 0 0] This works if default player is player 1, and then spawns player 2. Does not seem to work with 5.1.1 either
  (Variables|Default|SetDefaultPawnClass "/Game/GameBehaviour/Characters/Player/BP_Player2.BP_Player2_C")
  (Class|GameplayStatics|CreatePlayer -1))

(event EventBeginPlay
  (CallFunction|SpawnPlayers)
  (bind _asbp_player_1 (Utilities|Casting|CastToBP_Player1 (Game|GetPlayerCharacter 0)))
  (Game|BindEventtoOnDestroyed _asbp_player_1 (delegate Custom|OnDestroyed_))
  (bind _asbp_player_2 (Utilities|Casting|CastToBP_Player2 (Game|GetPlayerCharacter 1)))
  (Game|BindEventtoOnDestroyed _asbp_player_2 (delegate Custom|OnDestroyed_)))

(fn ConstructionScript)

(fn Respawn)