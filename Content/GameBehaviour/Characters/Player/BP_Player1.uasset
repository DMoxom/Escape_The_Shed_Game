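; Player 1 character whose ability reverses destruction on objects the player aims at.
; IA_Ability fires a line trace from the follow camera, ignoring both players, and sends ReverseDestructionMessage to hits implementing BI_DestructionControl.
; A helper function projects the other player's location to test whether they are within this player's split-screen view.
; Older time-reversal timeline, wall-collision toggle and velocity clamps remain disconnected, leaving the BeginPlay wall reference effectively unused.
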(event Input|EnhancedActionEvents|EnhancedInputActionIA_Ability
  (params (ActionValue :type Boolean) (ElapsedSeconds :type Float%20%28double-precision%29) (TriggeredSeconds :type Float%20%28double-precision%29) (InputAction :type Input%20Action%20Object%20Reference :default "/Game/ThirdPerson/Characters/Input/Actions/IA_Ability.IA_Ability"))
  (bind _followcamera (Variables|Default|GetFollowCamera))
  (bind _returnvalue (Transformation|GetWorldLocation _followcamera))
  (:Triggered
    (bind _outhit (Collision|LineTraceByChannel _returnvalue (+ _returnvalue (* (Math|Vector|GetForwardVector _followcamera) 5e+03)) "TraceTypeQuery2" false (Utilities|Array|MakeArray self (Game|GetPlayerCharacter 1)) "ForDuration"))
    (if (Utilities|DoesObjectImplementInterface (.hitactor _outhit) "/Game/GameBehaviour/Destruction/BI_DestructionControl.BI_DestructionControl_C")
      (Class|BIDestructionControl|ReverseDestruction(Message) (.hitactor _outhit)))))

(event EventBeginPlay
  (|CallParentFunction)
  (bind _returnvalue (Actor|GetActorOfClass "/Game/GameBehaviour/Destruction/Wall/BP_BreakWallCollision.BP_BreakWallCollision_C"))
  (Variables|Default|SetWallCollision _returnvalue))

(event EventTick
  (params (DeltaSeconds :type Float%20%28single-precision%29)))

(fn ConstructionScript
  (|CallParentFunction))

(fn IsOtherPlayeronScreen
  (bind _returnvalue (Viewport|GetViewportSize))
  (bind _ownplayerindex (Variables|Default|GetOwnPlayerIndex))
  (bind _otherplayerindex (Variables|Default|GetOtherPlayerIndex))
  (bind _returnvalue_2 (Game|GetPlayerController _ownplayerindex))
  (bind _returnvalue_3 (Game|GetPlayerCharacter _otherplayerindex))
  (bind _returnvalue_4 (Transformation|GetActorLocation _returnvalue_3))
  (bind _screenlocation (Class|PlayerController|ProjectWorldLocationtoScreen _returnvalue_2 _returnvalue_4 false))
  (return (and (Math|Float|InRange(Float) (.x _screenlocation) 0.0 (/ (.x _returnvalue) (Variables|Default|GetSplitScreenWidth))) (Math|Float|InRange(Float) (.y _screenlocation) 0.0 (.y _returnvalue)))))