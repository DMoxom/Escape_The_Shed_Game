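; BP_WallClimbChecker is a trigger volume that marks where the second player character can wall climb.
; Shortly after BeginPlay it caches player index 1 as BP_Player2.
; When an actor tagged Player2 enters the box, it enables CanClimb on that player's BPWallClimb.
; On exit it disables climbing, restores walking movement and orient-rotation-to-movement, and calls ResetClimb.
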(event OnComponentBeginOverlap(Box)
  (params (OverlappedComponent :type Primitive%20Component%20Object%20Reference) (OtherActor :type Actor%20Object%20Reference) (OtherComp :type Primitive%20Component%20Object%20Reference) (OtherBodyIndex :type Integer) (bFromSweep :type Boolean) (SweepResult :type Hit%20Result%20Structure%20%28by%20ref%29))
  (if (Actor|ActorHasTag OtherActor "Player2")
    (Variables|/Game/GameBehaviour/Characters/Player/Blueprints/WallClimbing/BP_WallClimb.BP_WallClimb_C|SetcanClimb (Variables|/Game/GameBehaviour/Characters/Player/SplitScreen/BP_Player2.BP_Player2_C|GetBP_WallClimb (Variables|Default|GetAs%20BP%20Player%202)) true)))

(event OnComponentEndOverlap(Box)
  (params (OverlappedComponent :type Primitive%20Component%20Object%20Reference) (OtherActor :type Actor%20Object%20Reference) (OtherComp :type Primitive%20Component%20Object%20Reference) (OtherBodyIndex :type Integer))
  (bind _as_bp_player_2 (Variables|Default|GetAs%20BP%20Player%202))
  (bind _charactermovement (Variables|/Script/Engine.Character|GetCharacterMovement _as_bp_player_2))
  (if (Actor|ActorHasTag OtherActor "Player2")
    (Variables|/Game/GameBehaviour/Characters/Player/Blueprints/WallClimbing/BP_WallClimb.BP_WallClimb_C|SetcanClimb (Variables|/Game/GameBehaviour/Characters/Player/SplitScreen/BP_Player2.BP_Player2_C|GetBP_WallClimb (Variables|Default|GetAs%20BP%20Player%202)) false)
    (Pawn|Components|CharacterMovement|SetMovementMode _charactermovement "MOVE_Walking" 0)
    (Variables|/Script/Engine.CharacterMovementComponent|SetbOrientRotationToMovement _charactermovement true)
    (Default|ResetClimb (Variables|/Game/GameBehaviour/Characters/Player/SplitScreen/BP_Player2.BP_Player2_C|GetBP_WallClimb (Variables|Default|GetAs%20BP%20Player%202)))))

(event EventBeginPlay
  (Utilities|FlowControl|Delay 0.2)
  (bind _asbp_player_2 (Utilities|Casting|CastToBP_Player2 (Game|GetPlayerCharacter 1)))
  (Variables|Default|SetAs%20BP%20Player%202 _asbp_player_2))

(fn ConstructionScript)