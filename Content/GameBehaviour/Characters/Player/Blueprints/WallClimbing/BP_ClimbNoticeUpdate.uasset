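; BP_ClimbNoticeUpdate switches on-screen climb and release prompts based on the second player's wall-climbing state.
; BeginPlay creates both widgets and, after a short delay, caches player index 1 as BP_Player2.
; Tick polls its BPWallClimb, showing the climb notice while climbing off a ledge and the release notice while climbing on one.
; Leaving the climb removes only the climb notice.
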(event EventBeginPlay
  (bind _returnvalue (UserInterface|CreateWidget "/Game/GameBehaviour/Characters/Player/Blueprints/WallClimbing/WBP_ClimbNotice.WBP_ClimbNotice_C"))
  (Variables|Default|SetClimbNotice _returnvalue)
  (bind _returnvalue_2 (UserInterface|CreateWidget "/Game/GameBehaviour/Characters/Player/Blueprints/WallClimbing/WBP_ReleaseNotice.WBP_ReleaseNotice_C"))
  (Variables|Default|SetReleaseNotice _returnvalue_2)
  (Utilities|FlowControl|Delay 0.2)
  (bind _asbp_player_2 (Utilities|Casting|CastToBP_Player2 (Game|GetPlayerCharacter 1)))
  (Variables|Default|SetAs%20BP%20Player%202 _asbp_player_2))

(event EventTick
  (params (DeltaSeconds :type Float%20%28single-precision%29))
  (bind _climbnotice (Variables|Default|GetClimbNotice))
  (bind _as_bp_player_2 (Variables|Default|GetAs%20BP%20Player%202))
  (bind _releasenotice (Variables|Default|GetReleaseNotice))
  (bind _bp_wallclimb (Variables|/Game/GameBehaviour/Characters/Player/SplitScreen/BP_Player2.BP_Player2_C|GetBP_WallClimb _as_bp_player_2))
  (Utilities|IsValid _as_bp_player_2
    (:Is%20Valid
      (if (Variables|/Game/GameBehaviour/Characters/Player/Blueprints/WallClimbing/BP_WallClimb.BP_WallClimb_C|GetisClimbing _bp_wallclimb)
        (if (Variables|/Game/GameBehaviour/Characters/Player/Blueprints/WallClimbing/BP_WallClimb.BP_WallClimb_C|GetisOnLedge _bp_wallclimb)
          (Widget|RemovefromParent _climbnotice :!label _label)
          (if (Variables|/Game/GameBehaviour/Characters/Player/Blueprints/WallClimbing/BP_WallClimb.BP_WallClimb_C|GetisClimbing (Variables|/Game/GameBehaviour/Characters/Player/SplitScreen/BP_Player2.BP_Player2_C|GetBP_WallClimb (Variables|Default|GetAs%20BP%20Player%202)))
            (UserInterface|Viewport|AddtoViewport _releasenotice 0))
          (else
            (UserInterface|Viewport|AddtoViewport _climbnotice 0)
            (Widget|RemovefromParent _releasenotice)))
        (else
          (goto _label))))))