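; Wall climbing logic for the second player character, which it fetches shortly after play begins.
; While CanClimb is set, Tick traces forward; a hit component tagged "Climb" turns the player to the wall and, through a DoOnce, switches movement to Flying.
; Losing the wall, or pressing Left Ctrl to launch backward, restores walking.
; A second trace records IsOnLedge, but the climb-over montage logic is unconnected.
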(event Custom|ResetClimb
  (bind _as_bp_player_2 (Variables|Default|GetAs%20BP%20Player%202))
  (bind _as_bp_player_2_2 (Variables|Default|GetAs%20BP%20Player%202))
  (bind _charactermovement (Variables|/Script/Engine.Character|GetCharacterMovement _as_bp_player_2))
  (bind _charactermovement_2 (Variables|/Script/Engine.Character|GetCharacterMovement _as_bp_player_2_2))
  (Pawn|Components|CharacterMovement|SetMovementMode _charactermovement "MOVE_Walking" 0)
  (Variables|/Script/Engine.CharacterMovementComponent|SetbOrientRotationToMovement _charactermovement true)
  (Utilities|FlowControl|DoOnce false) ; enters at Reset
)

(event EventBeginPlay
  (Utilities|FlowControl|Delay 0.2)
  (bind _asbp_player_2 (Utilities|Casting|CastToBP_Player2 (Game|GetPlayerCharacter 1)))
  (Variables|Default|SetAs%20BP%20Player%202 _asbp_player_2))

(event EventTick
  (params (DeltaSeconds :type Float%20%28single-precision%29))
  (bind _as_bp_player_2 (Variables|Default|GetAs%20BP%20Player%202))
  (bind _as_bp_player_2_2 (Variables|Default|GetAs%20BP%20Player%202))
  (bind _as_bp_player_2_3 (Variables|Default|GetAs%20BP%20Player%202))
  (bind _returnvalue (Transformation|GetActorLocation _as_bp_player_2))
  (bind _capsulecomponent (Variables|/Script/Engine.Character|GetCapsuleComponent _as_bp_player_2_2))
  (bind _charactermovement (Variables|/Script/Engine.Character|GetCharacterMovement _as_bp_player_2_3))
  (bind _returnvalue_2 (Transformation|GetWorldLocation _capsulecomponent))
  (if (Variables|Default|GetcanClimb)
    (Utilities|IsValid (Variables|Default|GetAs%20BP%20Player%202)
      (:Is%20Valid
        (if (not (Variables|Default|GetisClimbingUp))
          (bind (_outhit _returnvalue_3) (Collision|LineTraceByChannel _returnvalue_2 (+ _returnvalue_2 (* (Math|Vector|GetForwardVector _capsulecomponent) 5e+01)) "TraceTypeQuery1" false 0 "ForDuration"))
          (if _returnvalue_3
            (bind _returnvalue_4 (Collision|LineTraceByChannel _returnvalue (+ (+ _returnvalue "0.000000,0.000000,110.000000") (* (Transformation|GetActorForwardVector _as_bp_player_2) 5e+01)) "TraceTypeQuery1" false 0 "ForDuration" true "(R=0.000000,G=0.047853,B=1.000000,A=1.000000)"))
            (Variables|Default|SetisOnLedge _returnvalue_4)
            (if (Components|ComponentHasTag (.hitcomponent _outhit) "Climb")
              (Transformation|SetActorRotation (Variables|Default|GetAs%20BP%20Player%202) (Math|Rotator|MakeRotator 0.0 0.0 (+ (.yaw (Math|Conversions|RotationFromXVector (.normal _outhit))) 1.8e+02)))
              (Utilities|FlowControl|DoOnce false
                (:Completed
                  (Variables|Default|SetisClimbing true)
                  (Variables|/Script/Engine.MovementComponent|SetVelocity _charactermovement "0, 0, 0")
                  (Pawn|Components|CharacterMovement|SetMovementMode _charactermovement "MOVE_Flying" 0)
                  (Variables|/Script/Engine.CharacterMovementComponent|SetbOrientRotationToMovement _charactermovement false))))
            (elif (Variables|Default|GetisClimbing)
              (Variables|Default|SetisClimbing false)
              (CallFunction|ResetClimb))))))))

(event Input|KeyboardEvents|R
  (params (Key :type Key%20Structure :default "None")))

(event Input|KeyboardEvents|LeftCtrl
  (params (Key :type Key%20Structure :default "None"))
  (bind _as_bp_player_2 (Variables|Default|GetAs%20BP%20Player%202))
  (bind _returnvalue (Transformation|GetActorForwardVector _as_bp_player_2))
  (bind _returnvalue_2 (* _returnvalue -2e+02))
  (:Pressed
    (if (Variables|Default|GetisClimbing)
      (Character|LaunchCharacter (Variables|Default|GetAs%20BP%20Player%202) (Math|Vector|MakeVector (.x _returnvalue_2) (.y _returnvalue_2) 0.0) false false)
      (Variables|Default|SetisClimbing false)
      (CallFunction|ResetClimb))))

(event Input|KeyboardEvents|W
  (params (Key :type Key%20Structure :default "None")))