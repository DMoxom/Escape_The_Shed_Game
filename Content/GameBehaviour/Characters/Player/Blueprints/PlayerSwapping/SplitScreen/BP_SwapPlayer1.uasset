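; BP_SwapPlayer1 swaps the pawns controlled by the first two local players in split screen.
; Shortly after BeginPlay, it caches the pawns possessed by player controllers 0 and 1.
; Pressing Z makes each controller possess the other's cached pawn.
; The cached references are never updated, so repeated presses reapply the same assignment rather than swapping back.
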(event EventBeginPlay
  (Utilities|FlowControl|Delay 0.2)
  (Variables|Default|SetPlayer1 (Pawn|GetControlledPawn (Game|GetPlayerController 0)))
  (Variables|Default|SetPlayer2 (Pawn|GetControlledPawn (Game|GetPlayerController 1))))

(event Input|KeyboardEvents|Z
  (params (Key :type Key%20Structure :default "None"))
  (:Pressed
    (Pawn|Possess (Game|GetPlayerController 0) (Variables|Default|GetPlayer2))
    (Pawn|Possess (Game|GetPlayerController 1) (Variables|Default|GetPlayer1))))