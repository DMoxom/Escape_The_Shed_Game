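; Side-scroll player-swapping Blueprint that exchanges the pawns of the two local players when Z is pressed.
; Shortly after BeginPlay it caches both controllers' pawns and the first BP_Camera in the level.
; Z makes each controller possess the other's original pawn, then points both views back at that shared camera.
; The cached pawns are never updated, so further presses do not swap back.
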(event EventBeginPlay
  (Utilities|FlowControl|Delay 0.2)
  (Variables|Default|SetPlayer1 (Pawn|GetControlledPawn (Game|GetPlayerController 0)))
  (Variables|Default|SetPlayer2 (Pawn|GetControlledPawn (Game|GetPlayerController 1)))
  (bind _outactors (Actor|GetAllActorsOfClass "/Game/GameBehaviour/Characters/Player/SideScroll/BP_Camera.BP_Camera_C"))
  (Variables|Default|SetCamera (Utilities|Array|Get(acopy) _outactors)))

(event Input|KeyboardEvents|Z
  (params (Key :type Key%20Structure :default "None"))
  (:Pressed
    (Pawn|Possess (Game|GetPlayerController 0) (Variables|Default|GetPlayer2))
    (Pawn|Possess (Game|GetPlayerController 1) (Variables|Default|GetPlayer1))
    (Game|Player|SetViewTargetwithBlend (Game|GetPlayerController 0) (Variables|Default|GetCamera) 0.0 "VTBlend_Linear" 0.0 false)
    (Game|Player|SetViewTargetwithBlend (Game|GetPlayerController 1) (Variables|Default|GetCamera) 0.0 "VTBlend_Linear" 0.0 false)))