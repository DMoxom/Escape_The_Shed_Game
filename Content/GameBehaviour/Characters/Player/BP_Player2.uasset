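; Player 2 character Blueprint for split-screen play, showing an edge-of-screen indicator that points toward the other player when they are off-screen.
; BeginPlay creates the indicator widget; each Tick projects the other player into screen space and tests it against this player's part of the viewport.
; Off-screen, the indicator is clamped within padded bounds and rotated using Atan2 between both players' screen positions; on-screen, a resettable DoOnce hides it.
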(event EventBeginPlay
  (|CallParentFunction)
  ;[1 1 1] Gets ScreenEdgeIndicator widget and adds it to viewport
  (bind _returnvalue (UserInterface|CreateWidget "/Game/GameBehaviour/Characters/Player/ScreenEdgeIndicator/WBP_ScreenEdgeIndicator2.WBP_ScreenEdgeIndicator2_C"))
  (bind _output_get (Variables|Default|SetScreen%20Edge%20Indicator _returnvalue))
  (UserInterface|Viewport|AddtoViewport _output_get 0))

(event EventTick
  (params (DeltaSeconds :type Float%20%28single-precision%29))
  (bind _returnvalue (Transformation|GetActorLocation))
  (bind _returnvalue_2 (Viewport|GetViewportSize))
  (bind _ownplayerindex (Variables|Default|GetOwnPlayerIndex))
  (bind _otherplayerindex (Variables|Default|GetOtherPlayerIndex))
  (bind _screen_edge_indicator (Variables|Default|GetScreen%20Edge%20Indicator))
  (bind _ownplayerindex_2 (Variables|Default|GetOwnPlayerIndex))
  (bind _otherplayerindex_2 (Variables|Default|GetOtherPlayerIndex))
  (bind _returnvalue_3 (Game|GetPlayerCharacter _otherplayerindex))
  (bind _returnvalue_4 (Game|GetPlayerController _ownplayerindex_2))
  (bind _returnvalue_5 (Game|GetPlayerController _ownplayerindex))
  (bind _returnvalue_6 (Game|GetPlayerCharacter _otherplayerindex_2))
  (bind _returnvalue_7 (Class|Widget|GetDesiredSize _screen_edge_indicator))
  (bind _returnvalue_8 (Transformation|GetActorLocation _returnvalue_6))
  (bind _returnvalue_9 (Transformation|GetActorLocation _returnvalue_3))
  (bind _screenposition (Class|GameplayStatics|ProjectWorldtoScreen _returnvalue_5 _returnvalue false))
  (bind _returnvalue_10 (/ _returnvalue_7 "(X=2.000000,Y=2.000000)"))
  (bind _screenposition_2 (Class|GameplayStatics|ProjectWorldtoScreen _returnvalue_5 _returnvalue_9 false))
  (bind _screenposition_3 (Class|GameplayStatics|ProjectWorldtoScreen _returnvalue_4 _returnvalue_8 false))
  (bind _returnvalue_11 (- _returnvalue_2 _returnvalue_10))
  (bind _returnvalue_12 (- _screenposition _screenposition_2))
  (bind _outdir (Class|KismetMathLibrary|ToDirectionandLength2D _returnvalue_12))
  ;[1 1 1] Checks if the other player is on the current screen
  (bind _return_value (CallFunction|IsOtherPlayeronScreen))
  (if _return_value
    ;[1 1 1] If other player is on the screen, hide the edge indicator (only does it once)
    (Utilities|FlowControl|DoOnce false :!label _label
      (:Completed
        (Widget|SetVisibility (Variables|Default|GetScreen%20Edge%20Indicator) "Hidden")))
    (else
      ;[1 1 1] If othe other player is off the screen, show the screen edge indicator
      (Widget|SetVisibility (Variables|Default|GetScreen%20Edge%20Indicator) "Visible")
      ;[1 1 1] Sets the position of the screen edge indicator
      (Class|UserWidget|SetPositioninViewport (Variables|Default|GetScreen%20Edge%20Indicator) (Math|Vector2D|MakeVector2D (Math|Float|Clamp(Float) (.x _screenposition_3) (+ (/ (.x _returnvalue_11) (Variables|Default|GetSplitScreenWidth)) (Variables|Default|GetxMinPadding)) (- (.x _returnvalue_11) (Variables|Default|GetxMaxPadding))) (Math|Float|Clamp(Float) (.y _screenposition_3) 0.0 (- (.y _returnvalue_11) (Variables|Default|GetyPadding)))) true)
      ;[1 1 1] Sets the rotation of the screen edge indicator
      (Class|Widget|SetRenderTransformAngle (Variables|Default|GetScreen%20Edge%20Indicator) (+ (Class|KismetMathLibrary|DegAtan2 (.y _outdir) (.x _outdir)) -9e+01))
      (goto _label Reset))))

(fn ConstructionScript
  (|CallParentFunction))

(fn IsOtherPlayeronScreen
  (bind _returnvalue (Viewport|GetViewportSize))
  (bind _ownplayerindex (Variables|Default|GetOwnPlayerIndex))
  (bind _otherplayerindex (Variables|Default|GetOtherPlayerIndex))
  (bind _returnvalue_2 (Game|GetPlayerController _ownplayerindex))
  (bind _returnvalue_3 (Game|GetPlayerCharacter _otherplayerindex))
  (bind _returnvalue_4 (Transformation|GetActorLocation _returnvalue_3))
  (bind _screenlocation (Class|PlayerController|ProjectWorldLocationtoScreen _returnvalue_2 _returnvalue_4 false))
  (return (and (Math|Float|InRange(Float) (.x _screenlocation) (/ (.x _returnvalue) (Variables|Default|GetSplitScreenWidth)) (.x _returnvalue)) (Math|Float|InRange(Float) (.y _screenlocation) 0.0 (.y _returnvalue)))))