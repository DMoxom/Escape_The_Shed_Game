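; BP_Player2_SideScroll is the side-scrolling Player 2 character, a child Blueprint that enables climbing on BeginPlay and adds ability and animation responses.
; The ability input sends a destruct message to the repairing object when destruction is allowed.
; Jump input plays a double-jump montage based on jump counter, falling velocity and wall-climb state.
; Dash input plays a dash montage unless the character is both climbing and dashing.
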(event Input|EnhancedActionEvents|EnhancedInputActionIA_Ability
  (params (ActionValue :type Boolean) (ElapsedSeconds :type Float%20%28double-precision%29) (TriggeredSeconds :type Float%20%28double-precision%29) (InputAction :type Input%20Action%20Object%20Reference :default "/Game/ThirdPerson/Characters/Input/Actions/IA_Ability.IA_Ability"))
  (:Triggered
    (if (Variables|Default|GetcanDestroy)
      (Class|BIDestructionControl|DestructObject(Message) (Variables|Default|GetrepairingObject) true))))

(event Input|EnhancedActionEvents|EnhancedInputActionIA_Dash
  (params (ActionValue :type Boolean) (ElapsedSeconds :type Float%20%28double-precision%29) (TriggeredSeconds :type Float%20%28double-precision%29) (InputAction :type Input%20Action%20Object%20Reference :default "/Game/ThirdPerson/Characters/Input/Actions/IA_Dash.IA_Dash"))
  ;[1 1 1] Dash Anim
  (:Started
    (if (not (and (Variables|Default|GetIsClimbing) (Variables|Default|GetDashing)))
      (Animation|Montage|PlayMontage (Variables|Character|GetMesh) "/Game/GameBehaviour/Characters/Player/Potson/Animations/Sequences/A_Potson_Dash_01_Montage.A_Potson_Dash_01_Montage"))))

(event Input|EnhancedActionEvents|EnhancedInputActionIA_Jump
  (params (ActionValue :type Boolean) (ElapsedSeconds :type Float%20%28double-precision%29) (TriggeredSeconds :type Float%20%28double-precision%29) (InputAction :type Input%20Action%20Object%20Reference :default "/Game/ThirdPerson/Characters/Input/Actions/IA_Jump.IA_Jump"))
  ;[0.2188 0.2188 0.2188] Double Jump
  (:Triggered
    (if (not (Variables|/Game/GameBehaviour/Characters/Player/Blueprints/WallClimbing/BP_WallClimb.BP_WallClimb_C|GetisClimbing (Variables|Default|GetBP_WallClimb)))
      (if (and (and (AI|Components|NavMovement|IsFalling (Variables|Character|GetCharacterMovement)) (<= (.Z (Math|Vector|BreakVector (Transformation|GetVelocity))) -25.0)) (== (Variables|Default|GetJumpCounter) 1.0))
        (Variables|Default|SetJumpCounter 3.0)
        (Animation|Montage|PlayMontage (Variables|Character|GetMesh) "/Game/GameBehaviour/Characters/Player/Furlock/Animations/Sequences/A_Furlock_Jump_DoubleJump_01_Montage.A_Furlock_Jump_DoubleJump_01_Montage" :!label _label)
        (elif (== (Variables|Default|GetJumpCounter) 2.0)
          (goto _label))))))

(event EventBeginPlay
  (|CallParentFunction)
  (Variables|Default|SetEnableClimbing true))

(event Collision|EventActorBeginOverlap
  (params (OtherActor :type Actor%20Object%20Reference))
  (|CallParentFunction OtherActor) ; This node is disabled and will not be called.\nDrag off pins to build functionality.
)

(event EventTick
  (params (DeltaSeconds :type Float%20%28single-precision%29)))

(fn ConstructionScript
  (|CallParentFunction))