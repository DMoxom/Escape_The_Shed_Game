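; Side-scrolling Player 1 character Blueprint that layers Potson's repair, double-jump and dash animations onto input actions.
; The ability input messages RepairingObject to repair when CanRepair is set, without restarting an already playing fix montage.
; Jump input plays the double-jump montage based on JumpCounter, also advancing the counter when the first case occurs during a fall.
; Dash input only plays its montage when not already Dashing; no movement is applied here.
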(event Input|EnhancedActionEvents|EnhancedInputActionIA_Ability
  (params (ActionValue :type Boolean) (ElapsedSeconds :type Float%20%28double-precision%29) (TriggeredSeconds :type Float%20%28double-precision%29) (InputAction :type Input%20Action%20Object%20Reference :default "/Game/ThirdPerson/Characters/Input/Actions/IA_Ability.IA_Ability"))
  (bind _mesh (Variables|Character|GetMesh))
  (:Triggered
    (if (Variables|Default|GetcanRepair)
      (Class|BIDestructionControl|RepairObject(Message) (Variables|Default|GetrepairingObject) true)
      (if (not (Animation|Montage|MontageIsPlaying (Components|SkeletalMesh|GetAnimInstance _mesh) "/Game/GameBehaviour/Characters/Player/Potson/Animations/Sequences/A_Potson_Fix_02_Montage1.A_Potson_Fix_02_Montage1"))
        (Animation|Montage|PlayMontage _mesh "/Game/GameBehaviour/Characters/Player/Potson/Animations/Sequences/A_Potson_Fix_02_Montage1.A_Potson_Fix_02_Montage1")))))

(event Input|EnhancedActionEvents|EnhancedInputActionIA_Dash
  (params (ActionValue :type Boolean) (ElapsedSeconds :type Float%20%28double-precision%29) (TriggeredSeconds :type Float%20%28double-precision%29) (InputAction :type Input%20Action%20Object%20Reference :default "/Game/ThirdPerson/Characters/Input/Actions/IA_Dash.IA_Dash"))
  ;[1 1 1] Dash Anim
  (:Started
    (if (not (Variables|Default|GetDashing))
      (Animation|Montage|PlayMontage 0 "/Game/GameBehaviour/Characters/Player/Potson/Animations/Sequences/A_Potson_Dash_01_Montage.A_Potson_Dash_01_Montage"))))

(event Input|EnhancedActionEvents|EnhancedInputActionIA_Jump
  (params (ActionValue :type Boolean) (ElapsedSeconds :type Float%20%28double-precision%29) (TriggeredSeconds :type Float%20%28double-precision%29) (InputAction :type Input%20Action%20Object%20Reference :default "/Game/ThirdPerson/Characters/Input/Actions/IA_Jump.IA_Jump"))
  ;[0.2188 0.2188 0.2188] Double Jump
  (:Triggered
    (if (and (and (AI|Components|NavMovement|IsFalling (Variables|Character|GetCharacterMovement)) (<= (.Z (Math|Vector|BreakVector (Transformation|GetVelocity))) -25.0)) (== (Variables|Default|GetJumpCounter) 1.0))
      (Variables|Default|SetJumpCounter 3.0)
      (Animation|Montage|PlayMontage (Variables|Character|GetMesh) "/Game/GameBehaviour/Characters/Player/Potson/Animations/Sequences/A_Potson_DoubleJump_01_Montage.A_Potson_DoubleJump_01_Montage" :!label _label)
      (elif (== (Variables|Default|GetJumpCounter) 2.0)
        (goto _label)))))

(event EventBeginPlay
  (|CallParentFunction) ; This node is disabled and will not be called.\nDrag off pins to build functionality.
)

(event Collision|EventActorBeginOverlap
  (params (OtherActor :type Actor%20Object%20Reference))
  (|CallParentFunction OtherActor) ; This node is disabled and will not be called.\nDrag off pins to build functionality.
)

(event EventTick
  (params (DeltaSeconds :type Float%20%28single-precision%29)))

(fn ConstructionScript
  (|CallParentFunction))