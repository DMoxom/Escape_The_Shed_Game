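; BP_Camera is a shared side-scroll camera that keeps a group of players framed.
; CameraSetup caches all BP_BasePlayer_SideScroll actors and sets IsGameStarted, which enables the Tick updates.
; Each Tick lerps the Sphere component toward the players' average location at a fixed per-frame alpha.
; It also sets the spring arm length to the largest pairwise player distance, clamped between minimum and maximum limits.
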(event EventBeginPlay)

(event Collision|EventActorBeginOverlap
  (params (OtherActor :type Actor%20Object%20Reference)))

(event EventTick
  (params (DeltaSeconds :type Float%20%28single-precision%29))
  (if (Variables|Default|GetisGameStarted)
    (CallFunction|UpdateCameraMovement)
    (CallFunction|UpdateSpringArmLength)))

(fn ConstructionScript)

(fn CameraSetup
  (Variables|Default|SetisGameStarted true)
  (bind _outactors (Actor|GetAllActorsOfClass "/Game/GameBehaviour/Characters/Player/SideScroll/BP_BasePlayer_SideScroll.BP_BasePlayer_SideScroll_C"))
  (Variables|Default|SetPlayers _outactors))

(fn UpdateCameraMovement
  (Variables|Default|SetPreviousLocation (Transformation|GetWorldLocation (Variables|Default|GetSphere)))
  (bind _returnvalue (Class|GameplayStatics|GetActorArrayAverageLocation (Variables|Default|GetPlayers)))
  (Transformation|SetWorldLocation (Variables|Default|GetSphere) (Math|Vector|Lerp(Vector) (Variables|Default|GetPreviousLocation) _returnvalue (Variables|Default|GetMoveSpeed)) false false))

(fn UpdateSpringArmLength
  (for (_array_element _array_index) (Variables|Default|GetPlayers)
    (Variables|Default|SetCurrentPlayer _array_element)
    (for _index (range (+ _array_index 1) (- (Utilities|Array|Length (Variables|Default|GetPlayers)) 1))
      (Utilities|Array|Add (Variables|Default|GetDistance) (Transformation|GetDistanceTo (Variables|Default|GetCurrentPlayer) (Utilities|Array|Get(acopy) (Variables|Default|GetPlayers) _index)))))
  (Variables|/Script/Engine.SpringArmComponent|SetTargetArmLength (Variables|Default|GetSpringArm) (Math|Float|Clamp(Float) (.MaxValue (Math|Float|MaxOfFloatArray (Variables|Default|GetDistance))) (Variables|Default|GetMinArmLength) (Variables|Default|GetMaxArmLength)))
  (Utilities|Array|Clear (Variables|Default|GetDistance)))