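; Split-screen edge indicator meant to show a player's position on the other player's screen, currently inactive as all its logic is disconnected from empty BeginPlay and Tick.
; The unwired nodes create a screen-edge widget, project SelfActor through the other player's controller, and clamp it to a left or right viewport half by player index.
; They also select a target character and rotate the widget by the projected direction between the two actors.
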(event EventBeginPlay)

(event EventTick
  (params (DeltaSeconds :type Float%20%28single-precision%29))
  ;[1 1 1] Checks what player the blueprint is attatched to
)