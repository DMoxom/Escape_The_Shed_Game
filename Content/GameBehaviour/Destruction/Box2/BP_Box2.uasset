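; BP_Box2 is a destructible box that players can select, highlight and destroy, built from pre-fractured fragment meshes.
; Selection updates the two players' repair and destroy flags from the box's destroyed state and enables custom-depth highlighting.
; Destruction plays a timeline that drives a material scalar on every fragment, whose shared pivot parameter is set at BeginPlay.
; RepairObject is empty, with the timeline-reversal logic left unconnected.
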(event EventBeginPlay
  (bind _sm_box_low_geometrycollection1_1_ (Variables|Default|GetSM_Box_low_GeometryCollection1_1_))
  (bind _output_get (Variables|Default|SetDestruction%20Fragments (Utilities|Array|MakeArray _sm_box_low_geometrycollection1_1_ (Variables|Default|GetSM_Box_low_GeometryCollection1_2_) (Variables|Default|GetSM_Box_low_GeometryCollection1_3_) (Variables|Default|GetSM_Box_low_GeometryCollection1_4_) (Variables|Default|GetSM_Box_low_GeometryCollection1_5_) (Variables|Default|GetSM_Box_low_GeometryCollection1_6_) (Variables|Default|GetSM_Box_low_GeometryCollection1_7_) (Variables|Default|GetSM_Box_low_GeometryCollection1_8_) (Variables|Default|GetSM_Box_low_GeometryCollection1_9_) (Variables|Default|GetSM_Box_low_GeometryCollection1_10_) (Variables|Default|GetSM_Box_low_GeometryCollection1_11_) (Variables|Default|GetSM_Box_low_GeometryCollection1_12_) (Variables|Default|GetSM_Box_low_GeometryCollection1_13_) (Variables|Default|GetSM_Box_low_GeometryCollection1_14_) (Variables|Default|GetSM_Box_low_GeometryCollection1_15_) (Variables|Default|GetSM_Box_low_GeometryCollection1_16_) (Variables|Default|GetSM_Box_low_GeometryCollection1_17_) (Variables|Default|GetSM_Box_low_GeometryCollection1_18_) (Variables|Default|GetSM_Box_low_GeometryCollection1_19_) (Variables|Default|GetSM_Box_low_GeometryCollection1_20_) (Variables|Default|GetSM_Box_low_GeometryCollection1_21_))))
  (for _array_element _output_get
    (Rendering|Material|SetVectorParameterValueonMaterials _array_element "Pivot" (Transformation|GetWorldLocation _sm_box_low_geometrycollection1_1_))
    (Utilities|FlowControl|Delay 0.2)
    (bind _asbp_player_1 (Utilities|Casting|CastToBP_Player1 (Game|GetPlayerCharacter 0)))
    (Variables|Default|SetAs%20BP%20Player%201 _asbp_player_1)
    (bind _asbp_player_2 (Utilities|Casting|CastToBP_Player2 (Game|GetPlayerCharacter 1)))
    (Variables|Default|SetAs%20BP%20Player%202 _asbp_player_2)
    (Variables|Default|SetIsDestroyed false)))

(event EventObjectHighlight
  (params (CanBeInteractedWith :type Boolean))
  (if CanBeInteractedWith
    (if (Variables|Default|GetIsSelectedLocal)
      (for _array_element (Variables|Default|GetDestruction%20Fragments)
        (Rendering|SetRenderCustomDepth _array_element true)))))

(event EventSelectObject
  (Variables|Default|SetIsSelectedLocal true)
  (if (Variables|Default|GetIsDestroyed)
    (Variables|/Game/GameBehaviour/Characters/Player/BP_Player1.BP_Player1_C|SetCanBeRepaired (Variables|Default|GetAs%20BP%20Player%201) true)
    (Variables|/Game/GameBehaviour/Characters/Player/BP_Player2.BP_Player2_C|SetCanBeDestroyed (Variables|Default|GetAs%20BP%20Player%202) false)
    (else
      (Variables|/Game/GameBehaviour/Characters/Player/BP_Player1.BP_Player1_C|SetCanBeRepaired (Variables|Default|GetAs%20BP%20Player%201) false)
      (Variables|/Game/GameBehaviour/Characters/Player/BP_Player2.BP_Player2_C|SetCanBeDestroyed (Variables|Default|GetAs%20BP%20Player%202) true))))

(event EventRepairObject
  (params (isRepairable :type Boolean)))

(event EventDeselectObject
  (Variables|Default|SetIsSelectedLocal false)
  (for _array_element (Variables|Default|GetDestruction%20Fragments)
    (Rendering|SetRenderCustomDepth _array_element false)))

(event EventDestructObject
  (params (isDestructable :type Boolean))
  (if true
    (Variables|/Game/GameBehaviour/Characters/Player/BP_Player1.BP_Player1_C|SetCanBeRepaired (Variables|Default|GetAs%20BP%20Player%201) true)
    (Variables|/Game/GameBehaviour/Characters/Player/BP_Player2.BP_Player2_C|SetCanBeDestroyed (Variables|Default|GetAs%20BP%20Player%202) false)
    (Variables|Default|SetIsDestroyed true)
    (bind _newtrack_0 (Timeline|Destruction Play)
      (:Update
        (for _array_element (Variables|Default|GetDestruction%20Fragments)
          (Rendering|Material|SetScalarParameterValueonMaterials _array_element "Alpha 2" _newtrack_0))))))

(fn ConstructionScript)

(fn IsSelected
  (return false))