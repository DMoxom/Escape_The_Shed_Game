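; BP_BreakWallCollision1 is a collision volume for breakable walls, built around a Cube whose collision is switched by events.
; EnableCollision sets the Cube to query and physics collision, and DisableCollision sets it to no collision.
; Outside debugging, BeginPlay applies an invisible material.
; With IsDebugging set, both events also swap the Cube's material to show the current collision state.
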(event Custom|EnableCollision
  (Collision|SetCollisionEnabled (Variables|Default|GetCube) "QueryAndPhysics")
  (if (Variables|Default|GetIsDebugging)
    (Rendering|Material|SetMaterial (Variables|Default|GetCube) 0 "/Game/GameBehaviour/Destruction/M_Debugging.M_Debugging")))

(event Custom|DisableCollision
  (Collision|SetCollisionEnabled (Variables|Default|GetCube) "NoCollision")
  (if (Variables|Default|GetIsDebugging)
    (Rendering|Material|SetMaterial (Variables|Default|GetCube) 0 "/Game/GameBehaviour/Destruction/MI_DebuggingGreen.MI_DebuggingGreen")))

(event EventBeginPlay
  ;[1 1 1] Makes Wall Invisible if not debugging
  (if (not (Variables|Default|GetIsDebugging))
    (Rendering|Material|SetMaterial (Variables|Default|GetCube) 0 "/Game/GameBehaviour/Destruction/MI_DebuggingInvis.MI_DebuggingInvis")))

(fn ConstructionScript)