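; BP_Wall1 is a destructible wall built from twenty fragment meshes whose destruction is animated through material parameters.
; BeginPlay writes one fragment's world location to every mesh as a shared "Pivot" vector.
; ReverseDestruction alternately plays and reverses a timeline on each call, printing a debug message.
; The timeline track is split into two clamped halves driving "Alpha 1" then "Alpha 2", giving a sequential two-stage material animation.
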(event EventBeginPlay
  (bind _box_geometrycollection_sm_16_ (Variables|Default|GetBox_GeometryCollection_SM_16_))
  (Rendering|Material|SetVectorParameterValueonMaterials _box_geometrycollection_sm_16_ "Pivot" (Transformation|GetWorldLocation _box_geometrycollection_sm_16_)))

(event EventReverseDestruction
  (bind _box_geometrycollection_sm_16_ (Variables|Default|GetBox_GeometryCollection_SM_16_))
  (Development|PrintString "Activated")
  (Utilities|FlowControl|FlipFlop
    (:A
      (bind _newtrack_0 (Timeline|Destruction%20Reverse Play)
        (:Update
          (Rendering|Material|SetScalarParameterValueonMaterials _box_geometrycollection_sm_16_ "Alpha 1" (Math|Float|Clamp(Float) (* _newtrack_0 2.0)))
          (Rendering|Material|SetScalarParameterValueonMaterials _box_geometrycollection_sm_16_ "Alpha 2" (Math|Float|Clamp(Float) (- (* _newtrack_0 2.0) 1.0))))))
    (:B
      (Timeline|Destruction%20Reverse Reverse))))

(fn ConstructionScript)